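; Game mode for a local multiplayer drone race that spawns players, assigns start spots, creates their HUDs and starts or stops races.
; Each tick it bubble-sorts unfinished players by lap, checkpoint and distance into race rankings, plus a lap-independent circuit order for finding the player ahead.
; Final-level loading swaps out a streamed minigame, builds the level via GameData and starts a countdown.
; Three-player games add a spectator pawn as an extra player.
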(event `self.ReceiveBeginPlay`
  ;[1 1 1] Begin Play
  (`AkGameplayStatics.PostEventAtLocation` "/Game/Sounds/ambience/Play_IngameMusicRandomcontainer.Play_IngameMusicRandomcontainer")
  (bind _outactors (`GameplayStatics.GetAllActorsOfClass` "/Game/Blueprints/Level/LevelTransformGenerator.LevelTransformGenerator_C"))
  (set `self.LevelTransformGen` (`KismetArrayLibrary.Array_Get` _outactors))
  (bind _numberofplayers (`self.GetNumberOfPlayers`))
  (set `self.NumberOfPlayers` _numberofplayers)
  (`self.CreatePlayers` _numberofplayers)
  (`self.CreatePlayerHUDs` _numberofplayers)
  (bind _returnvalue (`|CreateWidget` "/Game/HUD/MiniMap.MiniMap_C"))
  (`UserWidget.AddToViewport` _returnvalue 9500))

(event `self.ReceiveTick`
  (params (DeltaSeconds :type "Float (single-precision)"))
  (bind _startranking (`self.StartRanking`))
  ;[1 1 1] Tick
  (while (> (`KismetArrayLibrary.Array_Length` (`self.StartRanking`)) 0)
    (if (`KismetArrayLibrary.Array_IsValidIndex` _startranking)
      (`KismetArrayLibrary.Array_Remove` _startranking)))
  (for _index (range (`self.NumberOfPlayers`))
    (if (not (`KismetArrayLibrary.Array_Contains` (`self.FinishedPlayers`) _index))
      (`KismetArrayLibrary.Array_Add` (`self.StartRanking`) _index)))
  (if (> (`KismetArrayLibrary.Array_Length` (`self.StartRanking`)) 1)
    (`self.GetPositionsInRace`)
    (`self.GetPositionsOnCircuit`)))

(event `StartGame`
  (params (CountdownInt :type Integer))
  ;[1 1 1] Start game
  (`self.SetActorTickEnabled` true)
  (for (_array_element _array_index) (`self.PlayerHUDs`)
    (`/Game/HUD/Player/PlayerHUD.StartCountdownAn` _array_element CountdownInt "Go!")
    (bind _asquadcopter_pawn (cast `/Game/Blueprints/Quadcopter/QuadcopterPawn` (`GameplayStatics.GetPlayerPawn` _array_index)))
    (`/Game/Blueprints/Quadcopter/QuadcopterPawn.BeginRace` _asquadcopter_pawn (`KismetMathLibrary.Conv_IntToDouble` (+ CountdownInt 1)))))

(event `StopGame`
  ;[1 1 1] Stop game
  (`self.SetActorTickEnabled` false))

(event `LoadFinalLevel`
  (if (`self.LevelLoadedFuse`)
    (set `self.LevelLoadedFuse` false)
    (`self.SetActorTickEnabled` false)
    (`KismetSystemLibrary.PrintString` "Load Level!" true false (struct :`G` 0.66 :`B` 1.0 :`A` 1.0) 6.0)
    (set `LevelStreaming.bShouldBeVisible` false (`GameplayStatics.GetStreamingLevel` (`self.MiniGame`)))
    (set `LevelStreaming.bShouldBeVisible` true (`GameplayStatics.GetStreamingLevel` (`self.LevelToLoad`)))
    (bind _asgame_data (cast `/Game/Blueprints/GameData` (`GameplayStatics.GetGameInstance`)))
    (`/Game/Blueprints/GameData.CreateLevel` _asgame_data (`KismetStringLibrary.Split` (`KismetStringLibrary.Conv_NameToString` (`self.LevelToLoad`)) "Data"))
    (`GameplayStatics.UnloadStreamLevel` (`self.MiniGame`))
    (`KismetSystemLibrary.Delay` 1.0)
    (bind _asgame_data_2 (cast `/Game/Blueprints/GameData` (`GameplayStatics.GetGameInstance`))
      (:`then`
        (`/Game/Blueprints/GameData.FadeIn` _asgame_data_2))
      (:`CastFailed`
        _))
    (`self.SetActorTickEnabled` true)
    (`self.StartGame` 3)
    (else
      (`KismetSystemLibrary.PrintString` "Game should have already started to load!!" true true (struct :`G` 0.66 :`B` 1.0 :`A` 1.0) 5.0))))

(event `self.ReceiveEndPlay`
  (params (EndPlayReason :type "EEndPlayReason Enum" :default "Destroyed"))
  (`KismetSystemLibrary.PrintString` "STOPPPPPPP" true false (struct :`R` 1.0 :`B` 0.080282 :`A` 1.0))
  (`AkGameplayStatics.PostEventAtLocation` "/Game/Sounds/ambience/Stop_IngameMusicRandomcontainer.Stop_IngameMusicRandomcontainer")
  (`AkGameplayStatics.PostEventAtLocation` "/Game/Sounds/drone/StopAllDrones.StopAllDrones"))

(fn `ChoosePlayerStart`
  (params (Player :type "Controller Object Reference"))
  (returns (ReturnValue :type "Actor Object Reference"))
  (bind _outactors (`GameplayStatics.GetAllActorsOfClass` "/Script/Engine.PlayerStart"))
  (for (_array_element _array_index) _outactors
    (if (!= (`PlayerStart.PlayerStartTag` _array_element) "Taken")
      (`|ExecutionSequence`
        (:`then_0`
          (break))
        (:`then_1`
          (`KismetSystemLibrary.PrintString` (`KismetStringLibrary.Concat_StrStr` "Place Player at StartPosition: " (`KismetStringLibrary.Conv_IntToString` _array_index)) true true (struct :`G` 0.66 :`B` 1.0 :`A` 1.0) 5.0))
        (:`then_2`
          (set `PlayerStart.PlayerStartTag` "Taken" _array_element)
          (return _array_element)))))
  (`KismetSystemLibrary.PrintString` "All spots taken spawn at deafult position." true true (struct :`R` 1.0 :`G` 0.464126 :`A` 1.0) 15.0)
  (return (`KismetArrayLibrary.Array_Get` _outactors)))

(fn `CreatePlayerHUDs`
  (params (PlayerCount :type Integer))
  (locals (playerhud :type "/Game/HUD/Player/PlayerHUD Object Reference"))
  (bind _playerhud (`local.playerhud`))
  (`KismetArrayLibrary.Array_Clear` (`self.PlayerHUDs`))
  (for _index (range PlayerCount)
    (`|ExecutionSequence`
      (:`then_0`
        (bind _returnvalue (`GameplayStatics.GetPlayerController` _index))
        (bind _returnvalue_2 (`|CreateWidget` "/Game/HUD/Player/PlayerHUD.PlayerHUD_C" _returnvalue))
        (bind _output_get (set `local.playerhud` _returnvalue_2))
        (`UserWidget.AddToPlayerScreen` _output_get 0))
      (:`then_1`
        (bind _ascopter_controller (cast `/Game/Blueprints/Quadcopter/CopterController` _returnvalue))
        (set `/Game/Blueprints/Quadcopter/CopterController.HUDWidget` (`local.playerhud`) _ascopter_controller))
      (:`then_2`
        (set `/Game/HUD/Player/PlayerHUD.PlayerID` _index _playerhud)
        (`KismetArrayLibrary.Array_Add` (`self.PlayerHUDs`) _playerhud)
        (bind _returnvalue_3 (`|CreateWidget` "/Game/HUD/Player/FinishHUD.FinishHUD_C" (`GameplayStatics.GetPlayerController` _index)))
        (`UserWidget.AddToPlayerScreen` _returnvalue_3 0)
        (set `/Game/HUD/Player/FinishHUD.PlayerID` _index _returnvalue_3)
        (`/Game/HUD/Player/FinishHUD.InitFinishHUD` _returnvalue_3)))))

(fn `CreatePlayers`
  (params (NumberOfPlayers :type Integer))
  (bind _outactors (`GameplayStatics.GetAllActorsOfClass` "/Game/Blueprints/Quadcopter/QuadcopterPawn.QuadcopterPawn_C"))
  (for _index (range (`KismetArrayLibrary.Array_Length` _outactors) NumberOfPlayers)
    (bind _returnvalue (`GameplayStatics.CreatePlayer` -1))
    (bind _asquadcopter_pawn (cast `/Game/Blueprints/Quadcopter/QuadcopterPawn` (`Controller.K2_GetPawn` _returnvalue)))
    (`/Game/Blueprints/Quadcopter/QuadcopterPawn.ChangeMaterial` _asquadcopter_pawn _index)
    (bind _ascopter_controller (cast `/Game/Blueprints/Quadcopter/CopterController` _returnvalue))
    (set `/Game/Blueprints/Quadcopter/CopterController.PlayerID` _index _ascopter_controller)
    (`KismetSystemLibrary.PrintString` (`KismetStringLibrary.Concat_StrStr` "Player created...." (`KismetStringLibrary.Conv_IntToString` _index)) true true (struct :`G` 0.66 :`B` 1.0 :`A` 1.0) 5.0))
  (if (== NumberOfPlayers 3)
    (bind _returnvalue_2 (`GameplayStatics.CreatePlayer` -1))
    (`self.K2_DestroyActor` (`Controller.K2_GetPawn` _returnvalue_2))
    (bind _returnvalue_3 (`|SpawnActorFromClass` "/Game/Blueprints/Spectator/SpectatorPawnForThirdPlayer.SpectatorPawnForThirdPlayer_C" (`KismetMathLibrary.MakeTransform` (0.0 0.0 0.0) (struct :`Pitch` 5.0 :`Roll` 50.0)) "AlwaysSpawn" "OverrideRootScale" _returnvalue_2))
    (`Controller.Possess` _returnvalue_2 _returnvalue_3)))

(fn `GetLeadingPlayer`
  (returns (PlayerID :type Integer))
  (return (`KismetArrayLibrary.Array_Get` (`self.RankingOnCircuit`))))

(fn `GetNumberOfPlayers`
  (returns (NumberOfPlayers :type Integer))
  (bind _asgame_data (cast `/Game/Blueprints/GameData` (`GameplayStatics.GetGameInstance`))
    (:`then`
      (return (`/Game/Blueprints/GameData.NumberOfPlayers` _asgame_data)))
    (:`CastFailed`
      (return -1))))

(fn `GetPlayerInFront`
  (params (PlayerID :type Integer))
  (returns (PlayerInFront :type Integer))
  (locals (InFront :type Integer))
  (bind _infront (`local.InFront`))
  (bind _returnvalue (`KismetArrayLibrary.Array_Find` (`self.PositionOnCircuit`) PlayerID))
  (if (> (`KismetArrayLibrary.Array_Length` (`self.PositionOnCircuit`)) 1)
    (if (== _returnvalue 0)
      (set `local.InFront` (`KismetArrayLibrary.Array_LastIndex` (`self.PositionOnCircuit`)))
      (else
        (bind _output_get (set `local.InFront` (- _returnvalue 1)))))
    (bind _returnvalue_2 (`self.GetPlayerQuadcopterPawn` _output_get :!label _label))
    (if (`/Game/Blueprints/Quadcopter/QuadcopterPawn.IsAlive` _returnvalue_2)
      (return (`KismetArrayLibrary.Array_Get` (`self.PositionOnCircuit`) (`local.InFront`)))
      (elif (== _infront 0)
        (set `local.InFront` (`KismetArrayLibrary.Array_LastIndex` (`self.PositionOnCircuit`)))
        (goto _label)
        (else
          (set `local.InFront` (- _infront 1))
          (goto _label))))
    (else
      (return PlayerID))))

(fn `GetPlayerPawn`
  (params (PlayerIndex :type Integer))
  (returns (ReturnValue :type "Pawn Object Reference"))
  (return (`GameplayStatics.GetPlayerPawn` PlayerIndex)))

(fn `GetPlayerPosition`
  (params (PlayerID :type Integer))
  (returns (Position :type Integer))
  (for _index (range (`KismetArrayLibrary.Array_Length` (`self.RankingInRace`)))
    (if (== PlayerID (`KismetArrayLibrary.Array_Get` (`self.RankingInRace`) _index))
      (break)))
  (return (+ _index 1)))

(fn `GetPlayerQuadcopterPawn`
  (params (PlayerIndex :type Integer))
  (returns (ReturnValue :type "/Game/Blueprints/Quadcopter/QuadcopterPawn Object Reference"))
  (bind _asquadcopter_pawn (cast `/Game/Blueprints/Quadcopter/QuadcopterPawn` (`GameplayStatics.GetPlayerPawn` PlayerIndex)))
  (return _asquadcopter_pawn))

(fn `GetPositionsInRace`
  (locals (Controller0 :type "/Game/Blueprints/Quadcopter/CopterController Object Reference") (Controller1 :type "/Game/Blueprints/Quadcopter/CopterController Object Reference") (swapped :type Boolean) (j :type Integer) (tmp :type Integer) (i :type Integer))
  (bind _controller0 (`local.Controller0`))
  (bind _rankingoncircuit (`self.RankingOnCircuit`))
  (bind _rankingoncircuit_2 (`self.RankingOnCircuit`))
  (bind _item (`KismetArrayLibrary.Array_Get` _rankingoncircuit (`local.i`)))
  (bind _item_2 (`KismetArrayLibrary.Array_Get` _rankingoncircuit (+ (`local.i`) 1)))
  (bind _returnvalue (`self.K2_GetActorLocation` (`KismetArrayLibrary.Array_Get` (`/Game/Blueprints/Quadcopter/CopterController.Checkpoints` _controller0) (`/Game/Blueprints/Quadcopter/CopterController.NextCheckpoint` _controller0))))
  (set `self.RankingOnCircuit` (`self.StartRanking`))
  (bind _output_get (set `local.swapped` true))
  (set `local.j` 0)
  (while _output_get
    (set `local.swapped` false)
    (`/Engine/EditorBlueprintResources/StandardMacros.IncrementInt` (`local.j`)
      (:`  `
        (for _index (range (+ (- (`KismetArrayLibrary.Array_Length` (`self.RankingOnCircuit`)) 2) 1))
          ;[1 1 1] Compare 2 Players and sort in temporary Array
          (set `local.i` _index)
          (`|ExecutionSequence`
            (:`then_0`
              (bind _ascopter_controller (cast `/Game/Blueprints/Quadcopter/CopterController` (`GameplayStatics.GetPlayerController` _item)))
              (set `local.Controller0` _ascopter_controller)
              (bind _ascopter_controller_2 (cast `/Game/Blueprints/Quadcopter/CopterController` (`GameplayStatics.GetPlayerController` _item_2)))
              (set `local.Controller1` _ascopter_controller_2))
            (:`then_1`
              (bind _lap (`/Game/Blueprints/Quadcopter/CopterController.GetCurrentLap` (`local.Controller0`)))
              (bind _lap_2 (`/Game/Blueprints/Quadcopter/CopterController.GetCurrentLap` (`local.Controller1`)))
              (if (> _lap _lap_2)
                _
                (elif (< _lap _lap_2)
                  (bind _output_get_2 (set `local.tmp` _item :!label _label))
                  (`KismetArrayLibrary.Array_Set` _rankingoncircuit_2 (`local.i`) _item_2)
                  (`KismetArrayLibrary.Array_Set` _rankingoncircuit_2 (+ (`local.i`) 1) _output_get_2)
                  (set `local.swapped` true)
                  (else
                    (bind _checkpoint (`/Game/Blueprints/Quadcopter/CopterController.GetNextCheckpoint` (`local.Controller0`)))
                    (bind _checkpoint_2 (`/Game/Blueprints/Quadcopter/CopterController.GetNextCheckpoint` (`local.Controller1`)))
                    (if (> _checkpoint _checkpoint_2)
                      _
                      (elif (< _checkpoint _checkpoint_2)
                        (goto _label)
                        (elif (not (< (`KismetMathLibrary.VSize` (- _returnvalue (`PlayerController.GetFocalLocation` _controller0))) (`KismetMathLibrary.VSize` (- _returnvalue (`PlayerController.GetFocalLocation` (`local.Controller1`))))))
                          (goto _label))))))))))
        ;[1 1 1] Combine already finished Players and Players on track
        (bind _output_get_3 (set `self.RankingInRace` (`self.FinishedPlayers`)))
        (`KismetArrayLibrary.Array_Append` _output_get_3 (`self.RankingOnCircuit`))))))

(fn `GetPositionsOnCircuit`
  (locals (Controller0 :type "/Game/Blueprints/Quadcopter/CopterController Object Reference") (Controller1 :type "/Game/Blueprints/Quadcopter/CopterController Object Reference") (swapped :type Boolean) (j :type Integer) (tmp :type Integer) (i :type Integer))
  (bind _controller0 (`local.Controller0`))
  (bind _positiononcircuit (`self.PositionOnCircuit`))
  (bind _positiononcircuit_2 (`self.PositionOnCircuit`))
  (bind _item (`KismetArrayLibrary.Array_Get` _positiononcircuit (`local.i`)))
  (bind _item_2 (`KismetArrayLibrary.Array_Get` _positiononcircuit (+ (`local.i`) 1)))
  (bind _returnvalue (`self.K2_GetActorLocation` (`KismetArrayLibrary.Array_Get` (`/Game/Blueprints/Quadcopter/CopterController.Checkpoints` _controller0) (`/Game/Blueprints/Quadcopter/CopterController.NextCheckpoint` _controller0))))
  (set `self.PositionOnCircuit` (`self.StartRanking`))
  (bind _output_get (set `local.swapped` true))
  (set `local.j` 0)
  (while _output_get
    (set `local.swapped` false)
    (`/Engine/EditorBlueprintResources/StandardMacros.IncrementInt` (`local.j`)
      (:`  `
        (for _index (range (+ (- (`KismetArrayLibrary.Array_Length` (`self.PositionOnCircuit`)) 2) 1))
          (set `local.i` _index)
          (`|ExecutionSequence`
            (:`then_0`
              (bind _ascopter_controller (cast `/Game/Blueprints/Quadcopter/CopterController` (`GameplayStatics.GetPlayerController` _item)))
              (set `local.Controller0` _ascopter_controller)
              (bind _ascopter_controller_2 (cast `/Game/Blueprints/Quadcopter/CopterController` (`GameplayStatics.GetPlayerController` _item_2)))
              (set `local.Controller1` _ascopter_controller_2))
            (:`then_1`
              (bind _checkpoint (`/Game/Blueprints/Quadcopter/CopterController.GetNextCheckpoint` (`local.Controller0`)))
              (bind _checkpoint_2 (`/Game/Blueprints/Quadcopter/CopterController.GetNextCheckpoint` (`local.Controller1`)))
              (if (> _checkpoint _checkpoint_2)
                _
                (elif (< _checkpoint _checkpoint_2)
                  (bind _output_get_2 (set `local.tmp` _item :!label _label))
                  (`KismetArrayLibrary.Array_Set` _positiononcircuit_2 (`local.i`) _item_2)
                  (`KismetArrayLibrary.Array_Set` _positiononcircuit_2 (+ (`local.i`) 1) _output_get_2)
                  (set `local.swapped` true)
                  (elif (not (< (`KismetMathLibrary.VSize` (- _returnvalue (`PlayerController.GetFocalLocation` _controller0))) (`KismetMathLibrary.VSize` (- _returnvalue (`PlayerController.GetFocalLocation` (`local.Controller1`))))))
                    (goto _label)))))))))))

(fn `PauseGame`
  (`self.SetRaceRunningForAllPlayers` false))

(fn `PlayerCountOnCircuit`
  (returns (Count :type Integer))
  (return (`KismetArrayLibrary.Array_Length` (`self.StartRanking`))))

(fn `PlayerFinished`
  (params (PlayerID :type Integer))
  (`KismetArrayLibrary.Array_Add` (`self.FinishedPlayers`) PlayerID))

(fn `ResumeGame`
  (`self.SetRaceRunningForAllPlayers` true))

(fn `SetLevelLoadedAndShowMessageToSkipMinigame`
  (bind _minimaphud (`self.MinimapHUD`))
  (`UserWidget.PlayAnimation` _minimaphud (`/Game/HUD/MiniGameStartNextLevel.Blinking` _minimaphud) 0.0 0 "Forward" 1.0)
  (set `self.LevelLoaded` true))

(fn `SetRaceRunningForAllPlayers`
  (params (IsRaceRunning :type Boolean))
  (for _index (range (`self.NumberOfPlayers`))
    (bind _ascopter_controller (cast `/Game/Blueprints/Quadcopter/CopterController` (`GameplayStatics.GetPlayerController` _index)))
    (set `/Game/Blueprints/Quadcopter/CopterController.IsRaceRunning` IsRaceRunning _ascopter_controller)))

(fn `UserConstructionScript`)