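; Player controller for a split-screen quadcopter race that tracks one player's checkpoints, laps and times.
; Trigger accepts only the next checkpoint in order, switches that player's checkpoint lights and counts laps.
; After the final lap it notifies the game mode, disables input and teleports the drone to its podium place.
; While racing, Tick advances the timer and projects the next checkpoint into the player's viewport for an edge-clamped HUD indicator.
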(event `self.ReceiveBeginPlay`
  (set `self.bForceFeedbackEnabled` true))

(event `self.ReceiveTick`
  (params (DeltaSeconds :type "Float (single-precision)"))
  (`|ExecutionSequence`
    (:`then_0`
      (if (`self.IsRaceRunning`)
        (set `self.ElapsedTime` (+ (`KismetMathLibrary.FromSeconds` DeltaSeconds) (`self.ElapsedTime`)))
        (`self.SetOffScreenIndicator`)))
    (:`then_1`
      ;[1 1 1] Debug
      (`KismetSystemLibrary.PrintString` (`KismetStringLibrary.Concat_StrStr` "Race running: " (`KismetStringLibrary.Conv_BoolToString` (`self.IsRaceRunning`)) " Time: " (`KismetStringLibrary.TimeSecondsToString` (/ (`KismetMathLibrary.GetTotalMilliseconds` (`self.ElapsedTime`)) 1000.0))) true false (struct :`G` 0.347 :`A` 1.0) 0.0))))

(fn `FindScreenEdgeLocationForWorldLocation`
  (params (InLocation :type "Vector Structure") (InViewportSize :type "Vector2D Structure") (InOffset :type "Vector2D Structure") (PlayerID :type Integer) (EdgePercent :type "Float (double-precision)"))
  (returns (OutScreenPosition :type "Vector2D Structure") (OutRotationAngleDegrees :type "Float (double-precision)") (IsOnScreen :type Boolean))
  (locals (mViewportSize :type "Vector2D Structure") (mViewportCenter :type "Vector2D Structure") (mInvert :type "Float (double-precision)") (mRotateInvert :type "Float (double-precision)") (mForward :type "Vector Structure" :default (0.0 0.0 0.0)) (mScreenPosition :type "Vector2D Structure") (mAngleRadians :type "Float (double-precision)" :default 0.0) (mCos :type "Float (double-precision)" :default 0.0) (mSin :type "Float (double-precision)" :default 0.0) (localm :type "Float (double-precision)" :default 0.0) (mScreenBounds :type "Vector2D Structure"))
  (bind (_mscreenposition_x _mscreenposition_y) (`KismetMathLibrary.BreakVector2D` (`local.mScreenPosition`)))
  (bind (_mviewportsize_x _mviewportsize_y) (`KismetMathLibrary.BreakVector2D` (`local.mViewportSize`)))
  (bind _mangleradians (`local.mAngleRadians`))
  (bind (_mscreenbounds_x _mscreenbounds_y) (`KismetMathLibrary.BreakVector2D` (`local.mScreenBounds`)))
  (bind _mscreenposition_x_2 (`KismetMathLibrary.BreakVector2D` (`local.mScreenPosition`)))
  (bind _mscreenbounds_x_2 (`KismetMathLibrary.BreakVector2D` (`local.mScreenBounds`)))
  (bind _mscreenbounds_x_3 (`KismetMathLibrary.BreakVector2D` (`local.mScreenBounds`)))
  (bind _returnvalue (/ _mscreenbounds_y (`local.localm`)))
  (bind _returnvalue_2 (* _mscreenbounds_x_3 (`local.localm`)))
  (set `local.mViewportSize` InViewportSize)
  (set `local.mViewportCenter` (/ InViewportSize 2.0))
  (set `local.mInvert` 1.0)
  (set `local.mRotateInvert` 0.0)
  (set `local.mForward` (`KismetMathLibrary.GetForwardVector` (`PlayerCameraManager.GetCameraRotation` (`self.PlayerCameraManager`))))
  (bind _output_get (set `local.mScreenPosition` (+ (`WidgetLayoutLibrary.ProjectWorldLocationToWidgetPosition` self InLocation) InOffset)))
  (if (== (`KismetMathLibrary.BreakVector2D` _output_get) 0.0)
    (set `local.mScreenPosition` (+ InOffset (`WidgetLayoutLibrary.ProjectWorldLocationToWidgetPosition` null (`KismetMathLibrary.VLerp` InLocation (`self.GetFocalLocation` self) 10.0))))
    (set `local.mInvert` -1.0)
    (set `local.mRotateInvert` 180.0)
    (elif (and (>= _mscreenposition_x 0.0) (<= _mscreenposition_x _mviewportsize_x) (>= _mscreenposition_y 0.0) (<= _mscreenposition_y _mviewportsize_y))
      (return (`local.mScreenPosition`) 0.0 true)
      (else
        _)))
  (bind _output_get_2 (set `local.mScreenPosition` (- (`local.mScreenPosition`) (`local.mViewportCenter`))))
  (bind _output_get_3 (set `local.mAngleRadians` (- (`KismetMathLibrary.Atan2` (`.Y` (`KismetMathLibrary.BreakVector2D` _output_get_2)) (`KismetMathLibrary.BreakVector2D` _output_get_2)) (`KismetMathLibrary.DegreesToRadians` 90.0))))
  (set `local.mCos` (`KismetMathLibrary.Cos` _mangleradians))
  (set `local.mSin` (* (`KismetMathLibrary.Sin` _mangleradians) -1.0))
  (set `local.localm` (/ (`local.mCos`) (`local.mSin`)))
  (set `local.mScreenBounds` (* (`local.mViewportCenter`) EdgePercent))
  (if (> (`local.mCos`) 0.0)
    (set `local.mScreenPosition` (`KismetMathLibrary.MakeVector2D` _returnvalue _mscreenbounds_y))
    (else
      (set `local.mScreenPosition` (`KismetMathLibrary.MakeVector2D` (* _returnvalue -1.0) (* _mscreenbounds_y -1.0)))))
  (if (> _mscreenposition_x_2 _mscreenbounds_x_2)
    (set `local.mScreenPosition` (`KismetMathLibrary.MakeVector2D` _mscreenbounds_x_3 _returnvalue_2))
    (elif (< _mscreenposition_x_2 (* _mscreenbounds_x_2 -1.0))
      (set `local.mScreenPosition` (`KismetMathLibrary.MakeVector2D` (* _mscreenbounds_x_3 -1.0) (* _returnvalue_2 -1.0)))))
  (return (+ (* (`local.mScreenPosition`) (`local.mInvert`)) (`local.mViewportCenter`)) (+ (+ (`KismetMathLibrary.RadiansToDegrees` _output_get_3) 180.0) (`local.mRotateInvert`)) false))

(fn `GetCurrentLap`
  (returns (Lap :type Integer))
  (return (`self.Lap`)))

(fn `GetNextCheckpoint`
  (returns (Checkpoint :type Integer))
  (return (`self.NextCheckpoint`)))

(fn `GetNextCheckpointActor`
  (returns (NextCheckpoint :type "Actor Object Reference"))
  (return (`KismetArrayLibrary.Array_Get` (`self.Checkpoints`) (`self.NextCheckpoint`))))

(fn `InitToStartValues`
  (set `self.Lap` 1)
  (set `self.NextCheckpoint` 0)
  (`KismetArrayLibrary.Array_Clear` (`self.LapTimes`))
  (`KismetArrayLibrary.Array_Clear` (`self.CheckpointTimes`))
  (set `self.ElapsedTime` (`KismetMathLibrary.FromMilliseconds` 0.0))
  (set `self.IsRaceRunning` false)
  (set `self.Finished` false))

(fn `PlaceDroneOnActorWithTag`
  (params (Tag :type Name))
  (bind _returnvalue (`self.K2_GetPawn`))
  (bind _outactors (`GameplayStatics.GetAllActorsWithTag` Tag))
  (if (== (`KismetArrayLibrary.Array_Length` _outactors) 1)
    (`self.SetActorEnableCollision` _returnvalue false)
    (bind _returnvalue_2 (`self.K2_TeleportTo` _returnvalue (.location (`self.GetTransform` (`KismetArrayLibrary.Array_Get` _outactors))) (.rotation (`self.GetTransform` (`KismetArrayLibrary.Array_Get` _outactors)))))
    (`self.SetActorEnableCollision` true)
    (if (not _returnvalue_2)
      (`KismetSystemLibrary.PrintString` "Actor couldn't fit" true true (struct :`R` 1.0 :`B` 0.061032 :`A` 1.0) 20.0))
    (bind _asquadcopter_pawn (cast `/Game/Blueprints/Quadcopter/QuadcopterPawn` _returnvalue))
    (`CameraComponent.SetPostProcessBlendWeight` (`/Game/Blueprints/Quadcopter/QuadcopterPawn.Camera` _asquadcopter_pawn) 0.0)
    (else
      (`KismetSystemLibrary.PrintString` "No Podium Place Actor found. Tag them FirstPlace, SecondPlace, ThirdPlace and FourthPlace" true true (struct :`R` 1.0 :`A` 1.0) 20.0))))

(fn `ResetToLastCheckpoint`
  (params (Pawn :type "Actor Object Reference"))
  (locals (LastCheckpoint :type Integer))
  (bind _nextcheckpoint (`self.NextCheckpoint`))
  (bind _item (`KismetArrayLibrary.Array_Get` (`self.Checkpoints`) (`local.LastCheckpoint`)))
  (bind (_returnvalue_roll _returnvalue_pitch _returnvalue_yaw) (`KismetMathLibrary.BreakRotator` (`self.K2_GetActorRotation` _item)))
  (if (== _nextcheckpoint 0)
    (set `local.LastCheckpoint` (- (`KismetArrayLibrary.Array_Length` (`self.Checkpoints`)) 1))
    (else
      (set `local.LastCheckpoint` (- _nextcheckpoint 1))))
  (`self.K2_SetActorLocationAndRotation` Pawn (`self.K2_GetActorLocation` _item) (`KismetMathLibrary.MakeRotator` 0.0 0.0 (+ _returnvalue_yaw -90.0)) false true))

(fn `SetOffScreenIndicator`
  (locals (ViewPort :type "Vector2D Structure" :default (0.0 0.0)) (Offset :type "Vector2D Structure"))
  (bind _asgame_data (cast `/Game/Blueprints/GameData` (`GameplayStatics.GetGameInstance`)))
  (bind _nextcheckpoint (`self.GetNextCheckpointActor`))
  (bind _ascheckpoint (cast `/Game/Blueprints/Checkpoint/Checkpoint` _nextcheckpoint))
  (if (== (`/Game/Blueprints/GameData.NumberOfPlayers` _asgame_data) 2)
    (set `local.ViewPort` (960.0 1080.0))
    (if (== (`self.PlayerID`) 0)
      (set `local.Offset` (0.0 0.0))
      (else
        (set `local.Offset` (960.0 0.0))))
    (else
      (set `local.ViewPort` (960.0 540.0))
      (if (== (`self.PlayerID`) 0)
        (set `local.Offset` (0.0 0.0))
        (elif (== (`self.PlayerID`) 1)
          (set `local.Offset` (960.0 0.0))
          (elif (== (`self.PlayerID`) 2)
            (set `local.Offset` (0.0 540.0))
            (else
              (set `local.Offset` (960.0 540.0))))))))
  (bind (_outscreenposition _outrotationangledegrees _bisonscreen) (`HUDBlueprintLibrary.FindScreenEdgeLocationForWorldLocation` (`self.K2_GetActorLocation` _ascheckpoint) (`local.ViewPort`) (`local.Offset`) (`self.PlayerID`) 0.9))
  (`/Game/HUD/Player/PlayerHUD.UpdateNextCheckpointIndicator` (`self.HUDWidget`) _outscreenposition _outrotationangledegrees _bisonscreen))

(fn `Trigger`
  (params (Checkpoint :type "Actor Object Reference"))
  (locals (NewLocalVar_0 :type Name :default "FirstPlace"))
  (if (`self.Finished`)
    _
    (elif (== Checkpoint (`KismetArrayLibrary.Array_Get` (`self.Checkpoints`) (`self.NextCheckpoint`)))
      (bind _asquadcopter_pawn (cast `/Game/Blueprints/Quadcopter/QuadcopterPawn` (`self.K2_GetPawn`)))
      (`ActorComponent.Activate` (`/Game/Blueprints/Quadcopter/QuadcopterPawn.EventRing` _asquadcopter_pawn) true)
      (bind _ascheckpoint (cast `/Game/Blueprints/Checkpoint/Checkpoint` (`KismetArrayLibrary.Array_Get` (`self.Checkpoints`) (`self.NextCheckpoint`))))
      (`/Game/Blueprints/Checkpoint/Checkpoint.Dark` _ascheckpoint (`self.PlayerID`))
      ;[1 1 1] Next Checkpoint
      (bind _result (`/Engine/EditorBlueprintResources/StandardMacros.IncrementInt` (`self.NextCheckpoint`)) ; Choose next Checkpoint
        (:`  `
          (if (>= _result (`KismetArrayLibrary.Array_Length` (`self.Checkpoints`)))
            (`KismetArrayLibrary.Array_Add` (`self.LapTimes`) (`self.ElapsedTime`))
            (set `self.ElapsedTime` (`KismetMathLibrary.FromMilliseconds` 0.0))
            (set `self.NextCheckpoint` 0)
            (bind _result_2 (`/Engine/EditorBlueprintResources/StandardMacros.IncrementInt` (`self.Lap`))
              (:`  `
                (if (> _result_2 (`self.MaxLaps`))
                  (set `self.Finished` true)
                  (bind _asbp_drone_racer_gm (cast `/Game/GameMode/BP_DroneRacerGM` (`GameplayStatics.GetGameMode`)))
                  (`/Game/GameMode/BP_DroneRacerGM.PlayerFinished` _asbp_drone_racer_gm (`self.PlayerID`))
                  (`GameplayStatics.PlaySound2D` "/Engine/EditorSounds/Notifications/CompileFailed.CompileFailed")
                  (`KismetSystemLibrary.PrintString` "finished" true true (struct :`G` 0.113725 :`B` 0.003922 :`A` 1.0))
                  (`self.DisableInput` (`self.K2_GetPawn`) null)
                  (`self.DisableInput` null)
                  (switch `int` (`/Game/HUD/Player/PlayerHUD.PlayerPosition` (`self.HUDWidget`))
                    (:`1`
                      (`self.PlaceDroneOnActorWithTag` "FirstPlace"))
                    (:`2`
                      (`self.PlaceDroneOnActorWithTag` "SecondPlace"))
                    (:`3`
                      (`self.PlaceDroneOnActorWithTag` "ThirdPlace"))
                    (:`4`
                      (`self.PlaceDroneOnActorWithTag` "FourthPlace")))
                  (else
                    (bind _ascheckpoint_2 (cast `/Game/Blueprints/Checkpoint/Checkpoint` (`KismetArrayLibrary.Array_Get` (`self.Checkpoints`) (`self.NextCheckpoint`)) :!label _label))
                    (`/Game/Blueprints/Checkpoint/Checkpoint.Light` _ascheckpoint_2 (`self.PlayerID`))))))
            (else
              (goto _label))))))))

(fn `UserConstructionScript`)