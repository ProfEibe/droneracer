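; Player quadcopter pawn with arcade flight, a pointer to the controller's current checkpoint, pickup spawning and per-player drone colors.
; Pitch, roll, yaw and throttle functions set interpolated speeds, with forward and sideways speed derived from current tilt.
; Tick applies local rotation, moves with sweep along flattened forward/right and actor up vectors, and aims the pointer.
; Throttle input also eases spring arm pitch for camera tilt.
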(event `self.ReceiveBeginPlay`
  (set `self.SpringArmDefaultRotation` (`SceneComponent.RelativeRotation` (`self.SpringArm`))))

(event `InputAxis|CameraYaw` :consume false
  (params (AxisValue :type "Float (single-precision)")))

(event `InputAxis|Throttle`
  (params (AxisValue :type "Float (single-precision)"))
  (if (`KismetMathLibrary.NearlyEqual_FloatFloat` AxisValue 0.0 0.001)
    (set `self.SpringArmYTargetRotation` (.pitch (`self.SpringArmDefaultRotation`)))
    (else
      (set `self.SpringArmYTargetRotation` (* AxisValue 35.0)))))

(event `self.ReceiveTick`
  (params (DeltaSeconds :type "Float (single-precision)"))
  (bind _springarm (`self.SpringArm`))
  (`|ExecutionSequence`
    (:`then_0`
      (`self.Tick` DeltaSeconds))
    (:`then_1`
      (`SceneComponent.K2_SetRelativeRotation` _springarm (`KismetMathLibrary.MakeRotator` (.roll (`SceneComponent.RelativeRotation` _springarm)) (`KismetMathLibrary.Lerp` (.pitch (`SceneComponent.RelativeRotation` _springarm)) (`self.SpringArmYTargetRotation`) DeltaSeconds) (.yaw (`SceneComponent.RelativeRotation` _springarm))) false false))))

(fn `ActivatePickup`
  (bind _pickupclass (`self.PickupClass`))
  (if (!= _pickupclass null)
    (`|SpawnActorFromClass` _pickupclass (`self.GetTransform`) "Undefined" "OverrideRootScale" self)))

(fn `ChangeMaterial`
  (params (PlayerNum :type Integer))
  (bind _drone (`self.Drone`))
  (switch `int` PlayerNum
    (:`Default`
      (bind _returnvalue (`KismetMaterialLibrary.CreateDynamicMaterialInstance` "/Game/Materials/MissileMaterial.MissileMaterial"))
      (`PrimitiveComponent.SetMaterial` _drone 0 _returnvalue))
    (:`0`
      (bind _returnvalue_2 (`KismetMaterialLibrary.CreateDynamicMaterialInstance` "/Game/Materials/DroneRed.DroneRed"))
      (`PrimitiveComponent.SetMaterial` _drone 0 _returnvalue_2))
    (:`1`
      (bind _returnvalue_3 (`KismetMaterialLibrary.CreateDynamicMaterialInstance` "/Game/Materials/DroneGreen.DroneGreen"))
      (`PrimitiveComponent.SetMaterial` _drone 0 _returnvalue_3))
    (:`2`
      (bind _returnvalue_4 (`KismetMaterialLibrary.CreateDynamicMaterialInstance` "/Game/Materials/DroneBlue.DroneBlue"))
      (`PrimitiveComponent.SetMaterial` _drone 0 _returnvalue_4))
    (:`3`
      (bind _returnvalue_5 (`KismetMaterialLibrary.CreateDynamicMaterialInstance` "/Game/Materials/DroneYellow.DroneYellow"))
      (`PrimitiveComponent.SetMaterial` _drone 0 _returnvalue_5))))

(fn `PitchCopter`
  (params (Value :type "Float (double-precision)"))
  (locals (TargetTilt :type "Float (double-precision)") (TiltDifference :type "Float (double-precision)") (TargetPitchSpeed :type "Float (double-precision)"))
  (bind (_returnvalue_roll _returnvalue_pitch) (`KismetMathLibrary.BreakRotator` (`self.K2_GetActorRotation`)))
  (bind _output_get (set `local.TargetTilt` (* Value (`self.MaxTargetTilt`))))
  (bind _output_get_2 (set `local.TiltDifference` (- _output_get _returnvalue_pitch)))
  (bind _output_get_3 (set `local.TargetPitchSpeed` (* _output_get_2 2.5)))
  (set `self.CurrentPitchSpeed` (`KismetMathLibrary.FInterpTo` (`self.CurrentPitchSpeed`) _output_get_3 (`GameplayStatics.GetWorldDeltaSeconds`) 7.0))
  (set `self.CurrentForwardSpeed` (* _returnvalue_pitch (`self.Acceleration`) -1.0)))

(fn `RollCopter`
  (params (Value :type "Float (double-precision)"))
  (locals (TargetTilt :type "Float (double-precision)") (TiltDifference :type "Float (double-precision)") (TargetRollSpeed :type "Float (double-precision)"))
  (bind _returnvalue_roll (`KismetMathLibrary.BreakRotator` (`self.K2_GetActorRotation`)))
  (bind _output_get (set `local.TargetTilt` (* Value (`self.MaxTargetTilt`))))
  (bind _output_get_2 (set `local.TiltDifference` (- _output_get _returnvalue_roll)))
  (bind _output_get_3 (set `local.TargetRollSpeed` (* _output_get_2 2.5)))
  (set `self.CurrentRollSpeed` (`KismetMathLibrary.FInterpTo` (`self.CurrentRollSpeed`) _output_get_3 (`GameplayStatics.GetWorldDeltaSeconds`) 8.0))
  (set `self.CurrentRightSpeed` (* _returnvalue_roll (`self.Acceleration`))))

(fn `ThrottleCopter`
  (params (Value :type "Float (double-precision)"))
  (set `self.CurrentUpSpeed` (`KismetMathLibrary.FInterpTo` (`self.CurrentUpSpeed`) (* Value 1000.0) (`GameplayStatics.GetWorldDeltaSeconds`) 3.5)))

(fn `Tick`
  (params (Delta :type "Float (double-precision)"))
  (locals (worldOffset :type "Vector Structure") (direction :type "Vector Structure") (deltaRotation :type "Rotator Structure"))
  (bind _returnvalue (`GameplayStatics.GetWorldDeltaSeconds`))
  (bind _returnvalue_2 (`GameplayStatics.GetWorldDeltaSeconds`))
  (bind _pointer (`self.Pointer`))
  (bind _drone (`self.Drone`))
  (bind (_returnvalue_x _returnvalue_y) (`KismetMathLibrary.BreakVector` (`SceneComponent.GetForwardVector` _drone)))
  (bind (_returnvalue_x_2 _returnvalue_y_2) (`KismetMathLibrary.BreakVector` (`SceneComponent.GetRightVector` _drone)))
  (`|ExecutionSequence`
    (:`then_0`
      ;[1 1 1] Rotation
      (bind _output_get (set `local.deltaRotation` (`KismetMathLibrary.MakeRotator` (* (`self.CurrentRollSpeed`) _returnvalue_2) (* (`self.CurrentPitchSpeed`) _returnvalue_2) (* (`self.CurrentYawSpeed`) _returnvalue_2))))
      (`self.K2_AddActorLocalRotation` _output_get))
    (:`then_1`
      ;[1 1 1] Translation
      (bind _output_get_2 (set `local.direction` (`KismetMathLibrary.MakeVector` _returnvalue_x _returnvalue_y)))
      (bind _output_get_3 (set `local.worldOffset` (* (`KismetMathLibrary.Normal` _output_get_2) (* (`self.CurrentForwardSpeed`) _returnvalue))))
      (bind _output_get_4 (set `local.direction` (`KismetMathLibrary.MakeVector` _returnvalue_x_2 _returnvalue_y_2)))
      (bind _output_get_5 (set `local.worldOffset` (+ _output_get_3 (* (`KismetMathLibrary.Normal` _output_get_4) (* (`self.CurrentRightSpeed`) _returnvalue)))))
      (bind _output_get_6 (set `local.direction` (`self.GetActorUpVector`)))
      (bind _output_get_7 (set `local.worldOffset` (+ _output_get_5 (* _output_get_6 (* (`self.CurrentUpSpeed`) _returnvalue)))))
      (`self.K2_AddActorWorldOffset` _output_get_7 true))
    (:`then_2`
      ;[1 1 1] Turn Arrow to next Checkpoint
      (bind _ascopter_controller (cast `/Game/Blueprints/Quadcopter/CopterController` (`self.GetController`)))
      (bind _item (`KismetArrayLibrary.Array_Get` (`/Game/Blueprints/Quadcopter/CopterController.Checkpoints` _ascopter_controller) (`/Game/Blueprints/Quadcopter/CopterController.Current` _ascopter_controller)))
      (if (`KismetSystemLibrary.IsValid` _item)
        (`SceneComponent.K2_SetWorldRotation` _pointer (`KismetMathLibrary.Conv_VectorToRotator` (- (`self.K2_GetActorLocation` _item) (`SceneComponent.K2_GetComponentLocation` _pointer))) true false)))))

(fn `UserConstructionScript`)

(fn `YawCopter`
  (params (Value :type "Float (double-precision)"))
  (set `self.CurrentYawSpeed` (`KismetMathLibrary.FInterpTo` (`self.CurrentYawSpeed`) (* Value (`self.Turnspeed`)) (`GameplayStatics.GetWorldDeltaSeconds`) 3.5)))