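; Checkpoint Blueprint with a front and back indicator light for each of four players.
; Light and Dark swap both of a player's lights to that player's lit or dark material, selected by a zero-based player number.
; Toggle reads the front light's current material to decide which of the two to call.
; A timed sequence that toggles each player's lights in turn sits disconnected in the EventGraph and never runs.
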(event `self.ReceiveTick`
  (params (DeltaSeconds :type "Float (single-precision)")))

(fn `Dark`
  (params (PlayerNumber :type Integer))
  (switch `int` PlayerNumber
    (:`0`
      (`PrimitiveComponent.SetMaterial` (`self.LightP1`) 0 "/Game/Flying/Meshes/LightMaterials/DarkP1.DarkP1")
      (`PrimitiveComponent.SetMaterial` (`self.BackLightP1`) 0 "/Game/Flying/Meshes/LightMaterials/DarkP1.DarkP1"))
    (:`1`
      (`PrimitiveComponent.SetMaterial` (`self.LightP2`) 0 "/Game/Flying/Meshes/LightMaterials/DarkP2.DarkP2")
      (`PrimitiveComponent.SetMaterial` (`self.BackLightP2`) 0 "/Game/Flying/Meshes/LightMaterials/DarkP2.DarkP2"))
    (:`2`
      (`PrimitiveComponent.SetMaterial` (`self.LightP3`) 0 "/Game/Flying/Meshes/LightMaterials/DarkP3.DarkP3")
      (`PrimitiveComponent.SetMaterial` (`self.BackLightP3`) 0 "/Game/Flying/Meshes/LightMaterials/DarkP3.DarkP3"))
    (:`3`
      (`PrimitiveComponent.SetMaterial` (`self.LightP4`) 0 "/Game/Flying/Meshes/LightMaterials/DarkP4.DarkP4")
      (`PrimitiveComponent.SetMaterial` (`self.BackLightP4`) 0 "/Game/Flying/Meshes/LightMaterials/DarkP4.DarkP4"))))

(fn `Light`
  (params (PlayerNumber :type Integer))
  (switch `int` PlayerNumber
    (:`0`
      (`PrimitiveComponent.SetMaterial` (`self.LightP1`) 0 "/Game/Flying/Meshes/LightMaterials/LightP1.LightP1")
      (`PrimitiveComponent.SetMaterial` (`self.BackLightP1`) 0 "/Game/Flying/Meshes/LightMaterials/LightP1.LightP1"))
    (:`1`
      (`PrimitiveComponent.SetMaterial` (`self.LightP2`) 0 "/Game/Flying/Meshes/LightMaterials/LightP2.LightP2")
      (`PrimitiveComponent.SetMaterial` (`self.BackLightP2`) 0 "/Game/Flying/Meshes/LightMaterials/LightP2.LightP2"))
    (:`2`
      (`PrimitiveComponent.SetMaterial` (`self.LightP3`) 0 "/Game/Flying/Meshes/LightMaterials/LightP3.LightP3")
      (`PrimitiveComponent.SetMaterial` (`self.BackLightP3`) 0 "/Game/Flying/Meshes/LightMaterials/LightP3.LightP3"))
    (:`3`
      (`PrimitiveComponent.SetMaterial` (`self.LightP4`) 0 "/Game/Flying/Meshes/LightMaterials/LightP4.LightP4")
      (`PrimitiveComponent.SetMaterial` (`self.BackLightP4`) 0 "/Game/Flying/Meshes/LightMaterials/LightP4.LightP4"))))

(fn `Toggle`
  (params (PlayerNumber :type Integer))
  (switch `int` PlayerNumber
    (:`0`
      (if (== (`PrimitiveComponent.GetMaterial` (`self.LightP1`) 0) "/Game/Flying/Meshes/LightMaterials/LightP1.LightP1")
        (`self.Dark` PlayerNumber :!label _label)
        (else
          (`self.Light` PlayerNumber :!label _label_2))))
    (:`1`
      (if (== (`PrimitiveComponent.GetMaterial` (`self.LightP2`) 0) "/Game/Flying/Meshes/LightMaterials/LightP2.LightP2")
        (goto _label)
        (else
          (goto _label_2))))
    (:`2`
      (if (== (`PrimitiveComponent.GetMaterial` (`self.LightP3`) 0) "/Game/Flying/Meshes/LightMaterials/LightP3.LightP3")
        (goto _label)
        (else
          (goto _label_2))))
    (:`3`
      (if (== (`PrimitiveComponent.GetMaterial` (`self.LightP4`) 0) "/Game/Flying/Meshes/LightMaterials/LightP4.LightP4")
        (goto _label)
        (else
          (goto _label_2))))))

(fn `UserConstructionScript`)