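; GameData is a game-wide data Blueprint, apparently a Game Instance, that manages screen fades and starts level creation.
; On Init it creates a Fade widget at a high Z-order and relays its animation-finished event through CallFadeFinished.
; FadeIn and FadeOut play that animation forward or in reverse, re-adding the widget if hidden.
; CreateLevel passes a level name and SubLevel to the first LevelTransformGenerator found, which also initializes players.
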(event `self.ReceiveInit`
  (bind _returnvalue (`|CreateWidget` "/Game/HUD/Fade.Fade_C"))
  (bind _output_get (set `self.FadeWidget` _returnvalue))
  (add `WidgetAnimation.OnAnimationFinished` (`/Game/HUD/Fade.Fade` _output_get) (delegate `CallFadeFinished`))
  (`UserWidget.AddToViewport` (`self.FadeWidget`) 9990))

(event `CallFadeFinished`
  (`self.FadeFinished`))

(fn `CreateLevel`
  (params (LevelName :type String))
  (bind _outactors (`GameplayStatics.GetAllActorsOfClass` "/Game/Blueprints/Level/LevelTransformGenerator.LevelTransformGenerator_C"))
  (`/Game/Blueprints/Level/LevelTransformGenerator.CreateLevelAndInitPlayers` (`KismetArrayLibrary.Array_Get` _outactors) LevelName (`self.SubLevel`)))

(fn `FadeIn`
  (`self.IsWidgetVisible`)
  (`/Game/HUD/Fade.StartFade` (`self.FadeWidget`) "Forward" 0.0))

(fn `FadeOut`
  (`self.IsWidgetVisible`)
  (`/Game/HUD/Fade.StartFade` (`self.FadeWidget`) "Reverse" 0.0))

(fn `IsWidgetVisible`
  (bind _fadewidget (`self.FadeWidget`))
  (`|ExecutionSequence`
    (:`then_0`
      (if (not (`Widget.IsVisible` _fadewidget))
        (`UserWidget.AddToViewport` _fadewidget 0)))
    (:`then_1`
      (return))))