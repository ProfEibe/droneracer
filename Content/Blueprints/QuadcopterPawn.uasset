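; Quadcopter pawn with simplified tilt-to-move flight, driven by pitch, roll, yaw and throttle functions.
; Pitch and roll ease their rotation rates toward target tilts, and the actual tilt sets forward and sideways speed.
; Tick applies local rotation, then a swept move along flattened mesh axes plus actor up for throttle.
; It also aims a Pointer component at the TriggerVolume referenced by CopterController.
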(event `self.ReceiveTick`
  (params (DeltaSeconds :type "Float (single-precision)"))
  (`self.Tick` DeltaSeconds))

(fn `PitchCopter`
  (params (Value :type "Float (double-precision)"))
  (locals (TargetTilt :type "Float (double-precision)") (TiltDifference :type "Float (double-precision)") (TargetPitchSpeed :type "Float (double-precision)"))
  (bind (_returnvalue_roll _returnvalue_pitch) (`KismetMathLibrary.BreakRotator` (`self.K2_GetActorRotation`)))
  (bind _output_get (set `local.TargetTilt` (* Value 20.0)))
  (bind _output_get_2 (set `local.TiltDifference` (- _output_get _returnvalue_pitch)))
  (bind _output_get_3 (set `local.TargetPitchSpeed` (* _output_get_2 2.5)))
  (set `self.CurrentPitchSpeed` (`KismetMathLibrary.FInterpTo` (`self.CurrentPitchSpeed`) _output_get_3 (`GameplayStatics.GetWorldDeltaSeconds`) 2.0))
  (set `self.CurrentForwardSpeed` (* _returnvalue_pitch (`self.Acceleration`) -1.0)))

(fn `RollCopter`
  (params (Value :type "Float (double-precision)"))
  (locals (TargetTilt :type "Float (double-precision)") (TiltDifference :type "Float (double-precision)") (TargetRollSpeed :type "Float (double-precision)"))
  (bind _returnvalue_roll (`KismetMathLibrary.BreakRotator` (`self.K2_GetActorRotation`)))
  (bind _output_get (set `local.TargetTilt` (* Value 20.0)))
  (bind _output_get_2 (set `local.TiltDifference` (- _output_get _returnvalue_roll)))
  (bind _output_get_3 (set `local.TargetRollSpeed` (* _output_get_2 2.5)))
  (set `self.CurrentRollSpeed` (`KismetMathLibrary.FInterpTo` (`self.CurrentRollSpeed`) _output_get_3 (`GameplayStatics.GetWorldDeltaSeconds`) 2.0))
  (set `self.CurrentRightSpeed` (* _returnvalue_roll (`self.Acceleration`))))

(fn `ThrottleCopter`
  (params (Value :type "Float (double-precision)"))
  (set `self.CurrentUpSpeed` (* Value 1000.0)))

(fn `Tick`
  (params (Delta :type "Float (double-precision)"))
  (locals (worldOffset :type "Vector Structure") (direction :type "Vector Structure") (deltaRotation :type "Rotator Structure"))
  (bind _returnvalue (`GameplayStatics.GetWorldDeltaSeconds`))
  (bind _pointer (`self.Pointer`))
  (bind _staticmesh (`self.StaticMesh`))
  (bind (_returnvalue_x _returnvalue_y) (`KismetMathLibrary.BreakVector` (`SceneComponent.GetForwardVector` _staticmesh)))
  (bind (_returnvalue_x_2 _returnvalue_y_2) (`KismetMathLibrary.BreakVector` (`SceneComponent.GetRightVector` _staticmesh)))
  ;[1 1 1] Rotation
  (bind _output_get (set `local.deltaRotation` (`KismetMathLibrary.MakeRotator` (* (`self.CurrentRollSpeed`) Delta) (* (`self.CurrentPitchSpeed`) Delta) (* (`self.CurrentYawSpeed`) Delta))))
  (`self.K2_AddActorLocalRotation` _output_get)
  ;[1 1 1] Translation
  (bind _output_get_2 (set `local.direction` (`KismetMathLibrary.MakeVector` _returnvalue_x _returnvalue_y)))
  (bind _output_get_3 (set `local.worldOffset` (* (`KismetMathLibrary.Normal` _output_get_2) (* (`self.CurrentForwardSpeed`) _returnvalue))))
  (bind _output_get_4 (set `local.direction` (`KismetMathLibrary.MakeVector` _returnvalue_x_2 _returnvalue_y_2)))
  (bind _output_get_5 (set `local.worldOffset` (+ _output_get_3 (* (`KismetMathLibrary.Normal` _output_get_4) (* (`self.CurrentRightSpeed`) _returnvalue)))))
  (bind _output_get_6 (set `local.direction` (`self.GetActorUpVector`)))
  (bind _output_get_7 (set `local.worldOffset` (+ _output_get_5 (* _output_get_6 (* (`self.CurrentUpSpeed`) _returnvalue)))))
  (`self.K2_AddActorWorldOffset` _output_get_7 true)
  (bind _ascopter_controller (cast `/Game/Blueprints/CopterController` (`GameplayStatics.GetPlayerController` 0)))
  (`SceneComponent.K2_SetWorldRotation` _pointer (`KismetMathLibrary.Conv_VectorToRotator` (- (`SceneComponent.K2_GetComponentLocation` (`Brush.BrushComponent` (`/Game/Blueprints/CopterController.TriggerVolume` _ascopter_controller))) (`SceneComponent.K2_GetComponentLocation` _pointer))) true false))

(fn `UserConstructionScript`
  (set `self.Acceleration` 50.0)
  (set `self.Turnspeed` 150.0))

(fn `YawCopter`
  (params (Value :type "Float (double-precision)"))
  (set `self.CurrentYawSpeed` (* Value (`self.Turnspeed`))))