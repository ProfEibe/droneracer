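; Checkpoint manager for a lap-based course, apparently for player one, that tracks the current checkpoint and lap count.
; Each Trigger call plays a sound, swaps the reached checkpoint's material and advances the index, wrapping to count a lap.
; One shared trigger volume moves to the next checkpoint with a 90-degree rotation offset, and that checkpoint's material changes to mark it active.
; Exceeding the lap limit plays an end sound instead of setting up another checkpoint.
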(fn `Trigger`
  (bind _checkpoints (`self.Checkpoints`))
  (bind _brushcomponent (`Brush.BrushComponent` (`self.TriggerVolumne`)))
  (bind _staticmeshcomponent (`StaticMeshActor.StaticMeshComponent` (`KismetArrayLibrary.Array_Get` _checkpoints (`self.Current`))))
  (`GameplayStatics.PlaySound2D` "/Engine/EditorSounds/Notifications/CompileSuccess.CompileSuccess")
  (`PrimitiveComponent.SetMaterial` _staticmeshcomponent 0 "/Engine/EditorMaterials/Camera/CineMat.CineMat")
  (bind _result (`/Engine/EditorBlueprintResources/StandardMacros.IncrementInt` (`self.Current`))
    (:`  `
      (if (>= _result (`KismetArrayLibrary.Array_Length` _checkpoints))
        (set `self.Current` 0)
        (bind _result_2 (`/Engine/EditorBlueprintResources/StandardMacros.IncrementInt` (`self.Lap`))
          (:`  `
            (if (> _result_2 (`self.MaxLaps`))
              (`GameplayStatics.PlaySound2D` "/Engine/EditorSounds/GamePreview/EndPlayInEditor.EndPlayInEditor")
              (else
                (`SceneComponent.K2_SetWorldTransform` _brushcomponent (`SceneComponent.K2_GetComponentToWorld` _staticmeshcomponent) false false :!label _label)
                (`SceneComponent.K2_AddRelativeRotation` _brushcomponent (struct :`Pitch` 90.0) false false)
                (`PrimitiveComponent.SetMaterial` _staticmeshcomponent 0 "/Engine/MapTemplates/Materials/BasicAsset01.BasicAsset01")))))
        (else
          (goto _label))))))

(fn `UserConstructionScript`)