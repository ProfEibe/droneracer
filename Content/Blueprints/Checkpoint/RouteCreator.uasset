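; RouteCreator builds race routes by spawning checkpoints and player starts from MapInfo entries matched by level name and number.
; On BeginPlay it creates the MiniGame route, waits a fixed delay, destroys it, then creates ElvenRuins using the GameData sub-level.
; Player starts receive index-based tags, and teardown removes only checkpoints.
; SetLaps is an empty stub, and a missing map prints an error.
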(event `self.ReceiveBeginPlay`
  (`self.CreateLevel` "MiniGame")
  (`KismetSystemLibrary.Delay` 9.0)
  (`self.DestroyLevel`)
  (bind _asgame_data (cast `/Game/Blueprints/GameData` (`GameplayStatics.GetGameInstance`)))
  (`self.CreateLevel` "ElvenRuins" (`/Game/Blueprints/GameData.SubLevel` _asgame_data)))

(fn `CreateLevel`
  (params (LevelName :type String) (LevelNumber :type Integer))
  (locals (FoundLevel :type Boolean))
  (bind _mapinfo (`self.MapInfo`))
  (set `local.FoundLevel` false)
  (for (_array_element _array_index) _mapinfo
    (bind (_name _levels) (break `/Game/Blueprints/Level/MapInfo` _array_element))
    (if (== LevelName _name)
      (`|ExecutionSequence`
        (:`then_0`
          (break))
        (:`then_1`
          (set `local.FoundLevel` true))
        (:`then_2`
          (bind (_checkpointtransforms _playerstarttransforms _laps) (break `/Game/Blueprints/Level/LevelInfo` (`KismetArrayLibrary.Array_Get` _levels LevelNumber)))
          (`self.SetCourse` _checkpointtransforms)
          (`self.SetPlayerStartPositions` _playerstarttransforms)
          (`self.SetLaps` _laps)))))
  (if (`local.FoundLevel`)
    _
    (elif (== (- (`KismetArrayLibrary.Array_Length` _mapinfo) 1) _array_index)
      (`KismetSystemLibrary.PrintString` "OHOH!!! Map Not Found!!!" true true (struct :`R` 1.0 :`A` 1.0) 20.0))))

(fn `DestroyLevel`
  (bind _checkpoints (`self.Checkpoints`))
  (for _array_element _checkpoints
    (`self.K2_DestroyActor` _array_element))
  (`KismetArrayLibrary.Array_Clear` _checkpoints))

(fn `SetCourse`
  (params (CheckpointTransforms :type "Array of Transform Structure"))
  (for _array_element CheckpointTransforms
    (bind _returnvalue (`|SpawnActorFromClass` "/Game/Blueprints/Checkpoint/Checkpoint.Checkpoint_C" _array_element "Undefined" "OverrideRootScale"))
    (`KismetArrayLibrary.Array_Add` (`self.Checkpoints`) _returnvalue)))

(fn `SetLaps`
  (params (Laps :type Integer)))

(fn `SetPlayerStartPositions`
  (params (PlayerStartTransforms :type "Array of Transform Structure"))
  (for (_array_element _array_index) PlayerStartTransforms
    (bind _returnvalue (`|SpawnActorFromClass` "/Script/Engine.PlayerStart" _array_element "AlwaysSpawn" "OverrideRootScale"))
    (`KismetArrayLibrary.Array_Add` (`Actor.Tags` _returnvalue) (`KismetStringLibrary.Conv_StringToName` (`KismetStringLibrary.Concat_StrStr` "Player" (`KismetStringLibrary.Conv_IntToString` _array_index))))))

(fn `UserConstructionScript`)