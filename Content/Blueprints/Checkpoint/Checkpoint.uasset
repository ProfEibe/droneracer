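; Race checkpoint actor that detects a quadcopter passing through its box and reports it to that copter's CopterController via Trigger.
; Only the pawn's CollisionBox counts, and a hit also posts a test Wwise event at the world origin.
; Light, Dark and Toggle swap front and back light materials for four players, while SetAsFinish activates four particle systems.
; A timed light-cycling test in the event graph is disconnected and never runs.
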(event `self.ReceiveBeginPlay`)

(event `self.ReceiveTick`
  (params (DeltaSeconds :type "Float (single-precision)")))

(event `self.Box.OnComponentBeginOverlap`
  (params (OverlappedComponent :type "PrimitiveComponent Object Reference") (OtherActor :type "Actor Object Reference") (OtherComp :type "PrimitiveComponent Object Reference") (OtherBodyIndex :type Integer) (bFromSweep :type Boolean) (SweepResult :type "HitResult Structure (by ref)"))
  ;[1 1 1] Check if hitted by Copter and not
  ; by arrow or camera
  (bind _asquadcopter_pawn (cast `/Game/Blueprints/Quadcopter/QuadcopterPawn` OtherActor))
  (if (== (`/Game/Blueprints/Quadcopter/QuadcopterPawn.CollisionBox` _asquadcopter_pawn) OtherComp)
    ;[1 1 1] Send to trigger function of Copter Controller
    (bind _ascopter_controller (cast `/Game/Blueprints/Quadcopter/CopterController` (`Pawn.GetController` _asquadcopter_pawn)))
    (`/Game/Blueprints/Quadcopter/CopterController.Trigger` _ascopter_controller self)
    (`AkGameplayStatics.PostEventAtLocation` "/Game/Sounds/Test_Event.Test_Event")))

(fn `Dark`
  (params (PlayerNumber :type Integer))
  (switch `int` PlayerNumber
    (:`0`
      (`PrimitiveComponent.SetMaterial` (`self.LightP1`) 0 "/Game/Materials/Checkpoints/DarkP1.DarkP1")
      (`PrimitiveComponent.SetMaterial` (`self.BackLightP1`) 0 "/Game/Materials/Checkpoints/DarkP1.DarkP1"))
    (:`1`
      (`PrimitiveComponent.SetMaterial` (`self.LightP2`) 0 "/Game/Materials/Checkpoints/DarkP2.DarkP2")
      (`PrimitiveComponent.SetMaterial` (`self.BackLightP2`) 0 "/Game/Materials/Checkpoints/DarkP2.DarkP2"))
    (:`2`
      (`PrimitiveComponent.SetMaterial` (`self.LightP3`) 0 "/Game/Materials/Checkpoints/DarkP3.DarkP3")
      (`PrimitiveComponent.SetMaterial` (`self.BackLightP3`) 0 "/Game/Materials/Checkpoints/DarkP3.DarkP3"))
    (:`3`
      (`PrimitiveComponent.SetMaterial` (`self.LightP4`) 0 "/Game/Materials/Checkpoints/DarkP4.DarkP4")
      (`PrimitiveComponent.SetMaterial` (`self.BackLightP4`) 0 "/Game/Materials/Checkpoints/DarkP4.DarkP4"))))

(fn `Light`
  (params (PlayerNumber :type Integer))
  (switch `int` PlayerNumber
    (:`0`
      (`PrimitiveComponent.SetMaterial` (`self.LightP1`) 0 "/Game/Materials/Checkpoints/LightP1.LightP1")
      (`PrimitiveComponent.SetMaterial` (`self.BackLightP1`) 0 "/Game/Materials/Checkpoints/LightP1.LightP1"))
    (:`1`
      (`PrimitiveComponent.SetMaterial` (`self.LightP2`) 0 "/Game/Materials/Checkpoints/LightP2.LightP2")
      (`PrimitiveComponent.SetMaterial` (`self.BackLightP2`) 0 "/Game/Materials/Checkpoints/LightP2.LightP2"))
    (:`2`
      (`PrimitiveComponent.SetMaterial` (`self.LightP3`) 0 "/Game/Materials/Checkpoints/LightP3.LightP3")
      (`PrimitiveComponent.SetMaterial` (`self.BackLightP3`) 0 "/Game/Materials/Checkpoints/LightP3.LightP3"))
    (:`3`
      (`PrimitiveComponent.SetMaterial` (`self.LightP4`) 0 "/Game/Materials/Checkpoints/LightP4.LightP4")
      (`PrimitiveComponent.SetMaterial` (`self.BackLightP4`) 0 "/Game/Materials/Checkpoints/LightP4.LightP4"))))

(fn `SetAsFinish`
  (`ActorComponent.SetActive` (`self.ParticleSystem`) true false)
  (`ActorComponent.SetActive` (`self.ParticleSystem1`) true false)
  (`ActorComponent.SetActive` (`self.ParticleSystem2`) true false)
  (`ActorComponent.SetActive` (`self.ParticleSystem3`) true false))

(fn `Toggle`
  (params (PlayerNumber :type Integer))
  (switch `int` PlayerNumber
    (:`0`
      (if (== (`PrimitiveComponent.GetMaterial` (`self.LightP2`) 0) "/Game/Materials/Checkpoints/LightP2.LightP2")
        (`self.Dark` PlayerNumber :!label _label)
        (else
          (`self.Light` PlayerNumber :!label _label_2))))
    (:`1`
      (if (== (`PrimitiveComponent.GetMaterial` (`self.LightP3`) 0) "/Game/Materials/Checkpoints/LightP1.LightP1")
        (goto _label)
        (else
          (goto _label_2))))
    (:`2`
      (if (== (`PrimitiveComponent.GetMaterial` (`self.LightP1`) 0) "/Game/Materials/Checkpoints/LightP3.LightP3")
        (goto _label)
        (else
          (goto _label_2))))
    (:`3`
      (if (== (`PrimitiveComponent.GetMaterial` (`self.LightP4`) 0) "/Game/Materials/Checkpoints/LightP4.LightP4")
        (goto _label)
        (else
          (goto _label_2))))))

(fn `UserConstructionScript`)