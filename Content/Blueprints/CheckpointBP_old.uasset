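; Checkpoint actor with four player lights and a shape built from spline mesh segments.
; The construction script adds a spline mesh between each pair of points on the Quarter spline and attaches it to RoundCheckpoint.
; Tick toggles the next player's light every quarter second, cycling through all four.
; Light, Dark and Toggle swap per-player materials, with Toggle reading the current material as the on/off state.
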(event `self.ReceiveTick`
  (params (DeltaSeconds :type "Float (single-precision)"))
  (bind _last (`self.last`))
  (bind _output_get (set `self.seconds` (+ DeltaSeconds (`self.seconds`))))
  (if (>= _output_get 0.25)
    (`self.Toggle` _last)
    (bind _result (`/Engine/EditorBlueprintResources/StandardMacros.IncrementInt` _last)
      (:`  `
        (if (>= _result 4)
          (set `self.last` 0))
        (set `self.seconds` (- (`self.seconds`) 0.25))))))

(fn `Dark`
  (params (PlayerNumber :type Integer))
  (switch `int` PlayerNumber
    (:`0`
      (`PrimitiveComponent.SetMaterial` (`self.LightP1`) 0 "/Game/Flying/Meshes/LightMaterials/DarkP1.DarkP1"))
    (:`1`
      (`PrimitiveComponent.SetMaterial` (`self.LightP2`) 0 "/Game/Flying/Meshes/LightMaterials/DarkP2.DarkP2"))
    (:`2`
      (`PrimitiveComponent.SetMaterial` (`self.LightP3`) 0 "/Game/Flying/Meshes/LightMaterials/DarkP3.DarkP3"))
    (:`3`
      (`PrimitiveComponent.SetMaterial` (`self.LightP4`) 0 "/Game/Flying/Meshes/LightMaterials/DarkP4.DarkP4"))))

(fn `Light`
  (params (PlayerNumber :type Integer))
  (switch `int` PlayerNumber
    (:`0`
      (`PrimitiveComponent.SetMaterial` (`self.LightP1`) 0 "/Game/Flying/Meshes/LightMaterials/LightP1.LightP1"))
    (:`1`
      (`PrimitiveComponent.SetMaterial` (`self.LightP2`) 0 "/Game/Flying/Meshes/LightMaterials/LightP2.LightP2"))
    (:`2`
      (`PrimitiveComponent.SetMaterial` (`self.LightP3`) 0 "/Game/Flying/Meshes/LightMaterials/LightP3.LightP3"))
    (:`3`
      (`PrimitiveComponent.SetMaterial` (`self.LightP4`) 0 "/Game/Flying/Meshes/LightMaterials/LightP4.LightP4"))))

(fn `Toggle`
  (params (PlayerNumber :type Integer))
  (switch `int` PlayerNumber
    (:`0`
      (if (== (`PrimitiveComponent.GetMaterial` (`self.LightP1`) 0) "/Game/Flying/Meshes/LightMaterials/LightP1.LightP1")
        (`self.Dark` PlayerNumber :!label _label)
        (else
          (`self.Light` PlayerNumber :!label _label_2))))
    (:`1`
      (if (== (`PrimitiveComponent.GetMaterial` (`self.LightP2`) 0) "/Game/Flying/Meshes/LightMaterials/LightP2.LightP2")
        (goto _label)
        (else
          (goto _label_2))))
    (:`2`
      (if (== (`PrimitiveComponent.GetMaterial` (`self.LightP3`) 0) "/Game/Flying/Meshes/LightMaterials/LightP3.LightP3")
        (goto _label)
        (else
          (goto _label_2))))
    (:`3`
      (if (== (`PrimitiveComponent.GetMaterial` (`self.LightP4`) 0) "/Game/Flying/Meshes/LightMaterials/LightP4.LightP4")
        (goto _label)
        (else
          (goto _label_2))))))

(fn `UserConstructionScript`
  (bind _myspline (`self.MySpline`))
  (set `self.MySpline` (`self.Quarter`))
  (for _index (range (+ (- (`SplineComponent.GetNumberOfSplinePoints` (`self.MySpline`)) 2) 1))
    (bind _returnvalue (`AddComponent|SplineMeshComponent_0` :`bManualAttachment` true))
    (`SceneComponent.K2_AttachToComponent` _returnvalue (`self.RoundCheckpoint`) "None" "KeepRelative" "KeepRelative" "KeepWorld" true)
    (bind (_location _tangent) (`SplineComponent.GetLocationAndTangentAtSplinePoint` _myspline _index "Local"))
    (bind (_location_2 _tangent_2) (`SplineComponent.GetLocationAndTangentAtSplinePoint` _myspline (+ _index 1) "Local"))
    (`SplineMeshComponent.SetStartAndEnd` _returnvalue _location _tangent _location_2 _tangent_2 true)))