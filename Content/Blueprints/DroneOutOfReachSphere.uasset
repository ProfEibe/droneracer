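; Trigger volume actor that marks the drone's reachable area and warns the player when the quadcopter leaves it.
; Leaving the overlap sets the pawn camera's post-process blend weight to full and starts a blinking out-of-reach message on the CopterController's HUD widget.
; Entering resets the blend weight to zero and stops the blinking, with both events sharing one helper function that filters for QuadcopterPawn.
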(event `self.ReceiveActorBeginOverlap`
  (params (OtherActor :type "Actor Object Reference"))
  (`self.SetBlendWeightAndBlinkingText` OtherActor true))

(event `self.ReceiveActorEndOverlap`
  (params (OtherActor :type "Actor Object Reference"))
  (`self.SetBlendWeightAndBlinkingText` OtherActor false 1.0 "Drone is out of Reach. Return..."))

(fn `SetBlendWeightAndBlinkingText`
  (params (Object :type "Object Object Reference") (DisableAnimation :type Boolean) (BlendWeight :type "Float (double-precision)") (BlinkingText :type Text))
  (bind _asquadcopter_pawn (cast `/Game/Blueprints/Quadcopter/QuadcopterPawn` Object)
    (:`then`
      (`CameraComponent.SetPostProcessBlendWeight` (`/Game/Blueprints/Quadcopter/QuadcopterPawn.Camera` _asquadcopter_pawn) BlendWeight)
      (bind _ascopter_controller (cast `/Game/Blueprints/Quadcopter/CopterController` (`Pawn.GetController` _asquadcopter_pawn))
        (:`then`
          (if DisableAnimation
            (bind _hudwidget (`/Game/Blueprints/Quadcopter/CopterController.HUDWidget` _ascopter_controller))
            (`/Game/HUD/Player/PlayerHUD.StopBlinking` _hudwidget)
            (else
              (`/Game/HUD/Player/PlayerHUD.StartBlinkingWithText` _hudwidget BlinkingText)))
          (return))
        (:`CastFailed`
          _)))
    (:`CastFailed`
      _))
  (return))

(fn `UserConstructionScript`)