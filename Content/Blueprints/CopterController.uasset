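; Quadcopter controller that passes player flight input to the pawn and contains checkpoint lap-race logic.
; Pitch, roll, throttle and yaw axes each cast the controlled pawn to QuadcopterPawn and call its matching function.
; Trigger advances checkpoint and lap counters, moving one reused trigger volume to the next checkpoint and swapping materials to mark it.
; Sounds signal checkpoint hits and race end, when the volume is destroyed.
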(event `InputAxis|Pitch`
  (params (AxisValue :type "Float (single-precision)"))
  (bind _asquadcopter_pawn (cast `/Game/Blueprints/QuadcopterPawn` (`self.K2_GetPawn`))
    (:`then`
      (`/Game/Blueprints/QuadcopterPawn.PitchCopter` _asquadcopter_pawn AxisValue))
    (:`CastFailed`
      (`KismetSystemLibrary.PrintString` "Quadcopterpawn not there!!" false false (struct :`R` 1.0 :`G` 0.012482 :`A` 1.0) 2.0 :!label _label))))

(event `self.ReceiveBeginPlay`)

(event `InputAxis|Roll`
  (params (AxisValue :type "Float (single-precision)"))
  (bind _asquadcopter_pawn (cast `/Game/Blueprints/QuadcopterPawn` (`self.K2_GetPawn`))
    (:`then`
      (`/Game/Blueprints/QuadcopterPawn.RollCopter` _asquadcopter_pawn AxisValue))
    (:`CastFailed`
      (goto _label))))

(event `InputAxis|Throttle`
  (params (AxisValue :type "Float (single-precision)"))
  (bind _asquadcopter_pawn (cast `/Game/Blueprints/QuadcopterPawn` (`self.K2_GetPawn`))
    (:`then`
      (`/Game/Blueprints/QuadcopterPawn.ThrottleCopter` _asquadcopter_pawn AxisValue))
    (:`CastFailed`
      (goto _label))))

(event `InputAxis|Yaw`
  (params (AxisValue :type "Float (single-precision)"))
  (bind _asquadcopter_pawn (cast `/Game/Blueprints/QuadcopterPawn` (`self.K2_GetPawn`))
    (:`then`
      (`/Game/Blueprints/QuadcopterPawn.YawCopter` _asquadcopter_pawn AxisValue))
    (:`CastFailed`
      (goto _label))))

(fn `Trigger`
  (params (Checkpoints :type "Array of StaticMeshActor Object Reference") (TriggerVolume :type "TriggerVolume Object Reference"))
  (bind _lap (`self.Lap`))
  (bind _brushcomponent (`Brush.BrushComponent` TriggerVolume))
  (bind _staticmeshcomponent (`StaticMeshActor.StaticMeshComponent` (`KismetArrayLibrary.Array_Get` Checkpoints (`self.Current`))))
  (set `self.TriggerVolume` TriggerVolume)
  (`GameplayStatics.PlaySound2D` "/Engine/EditorSounds/Notifications/CompileSuccess.CompileSuccess")
  (`PrimitiveComponent.SetMaterial` _staticmeshcomponent 0 "/Engine/EditorMaterials/Camera/CineMat.CineMat") ; Reset Material
  ;[1 1 1] Check where in race
  (bind _result (`/Engine/EditorBlueprintResources/StandardMacros.IncrementInt` (`self.Current`))
    (:`  `
      (if (>= _result (`KismetArrayLibrary.Array_Length` Checkpoints))
        ;[1 1 1] New Lap
        (set `self.Current` 0)
        (bind _result_2 (`/Engine/EditorBlueprintResources/StandardMacros.IncrementInt` _lap)
          (:`  `
            (if (> _result_2 (`self.MaxLaps`))
              ;[1 1 1] Race finished
              (`GameplayStatics.PlaySound2D` "/Engine/EditorSounds/Notifications/CompileFailed.CompileFailed")
              (`self.K2_DestroyActor` TriggerVolume)
              (else
                (`KismetSystemLibrary.PrintString` (`KismetStringLibrary.Concat_StrStr` "Runde " (`KismetStringLibrary.Conv_IntToString` _lap)) true true (struct :`G` 0.66 :`B` 1.0 :`A` 1.0) 5.0)
                ;[1 1 1] Set Trigger to next Checkpoint
                (`SceneComponent.K2_SetWorldTransform` _brushcomponent (`SceneComponent.K2_GetComponentToWorld` _staticmeshcomponent) false false :!label _label)
                (`SceneComponent.K2_AddRelativeRotation` _brushcomponent (struct :`Pitch` 90.0) false false)
                (`PrimitiveComponent.SetMaterial` _staticmeshcomponent 0 "/Engine/MapTemplates/Materials/BasicAsset01.BasicAsset01")))))
        (else
          (goto _label))))))

(fn `UserConstructionScript`)