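; EMP pickup effect actor that temporarily applies an EMP to the quadcopter pawns of players other than its owner.
; On BeginPlay it loops over the player count from GameData, calls ActivateEMP on each other pawn and stores those that return true.
; Tick counts down SecondsToLast, then deactivates the EMP on the stored pawns and destroys the actor.
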(event `self.ReceiveBeginPlay`
  (`KismetArrayLibrary.Array_Clear` (`self.OtherPlayerPawns`))
  (`KismetSystemLibrary.PrintString` "Start EMP" true true (struct :`R` 0.8282 :`B` 1.0 :`A` 1.0) 7.0)
  (bind _asquadcopter_pawn (cast `/Game/Blueprints/Quadcopter/QuadcopterPawn` (`self.GetOwner`)))
  (bind _asgame_data (cast `/Game/Blueprints/GameData` (`GameplayStatics.GetGameInstance`)))
  (for _index (range (`/Game/Blueprints/GameData.NumberOfPlayers` _asgame_data))
    (bind _asquadcopter_pawn_2 (cast `/Game/Blueprints/Quadcopter/QuadcopterPawn` (`GameplayStatics.GetPlayerPawn` _index)))
    (if (not (== _asquadcopter_pawn_2 _asquadcopter_pawn))
      (bind _activated (`/Game/Blueprints/Quadcopter/QuadcopterPawn.ActivateEMP` _asquadcopter_pawn_2))
      (if _activated
        (`KismetArrayLibrary.Array_Add` (`self.OtherPlayerPawns`) _asquadcopter_pawn_2)))))

(event `self.ReceiveTick`
  (params (DeltaSeconds :type "Float (single-precision)"))
  (bind _output_get (set `self.SecondsToLast` (- (`self.SecondsToLast`) DeltaSeconds)))
  (if (<= _output_get 0.0)
    (`KismetSystemLibrary.PrintString` "Done with emp!!" true true (struct :`R` 0.531298 :`B` 1.0 :`A` 1.0) 7.0)
    (for _array_element (`self.OtherPlayerPawns`)
      (`/Game/Blueprints/Quadcopter/QuadcopterPawn.DeactiveEMP` _array_element))
    (`self.K2_DestroyActor`)))

(fn `UserConstructionScript`)