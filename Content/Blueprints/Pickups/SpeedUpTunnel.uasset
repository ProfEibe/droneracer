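; Speed-up tunnel actor that pushes quadcopter pawns inside its BoostArea capsule along the actor's up vector.
; Overlap events maintain the list of captured copters, and Tick adds a boost to each one's MovementAlteringDraw.
; The boost scales MaxBoostFactor by capsule progress over length.
; The helper graphs hold axis-projection math measuring distance to the capsule's top end, but those expressions appear unconnected to any output.
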(event `self.ReceiveTick`
  (params (DeltaSeconds :type "Float (single-precision)"))
  (for _array_element (`self.CapturedCopters`)
    (bind _boostamount (`self.CalculateBoostAmount` _array_element))
    (set `/Game/Blueprints/Quadcopter/QuadcopterPawn.MovementAlteringDraw` (+ (* (`self.GetActorUpVector`) _boostamount) (`/Game/Blueprints/Quadcopter/QuadcopterPawn.MovementAlteringDraw` _array_element)) _array_element)))

(event `self.BoostArea.OnComponentBeginOverlap`
  (params (OverlappedComponent :type "PrimitiveComponent Object Reference") (OtherActor :type "Actor Object Reference") (OtherComp :type "PrimitiveComponent Object Reference") (OtherBodyIndex :type Integer) (bFromSweep :type Boolean) (SweepResult :type "HitResult Structure (by ref)"))
  ;[1 1 1] Capturing Pawns Code
  (bind _asquadcopter_pawn (cast `/Game/Blueprints/Quadcopter/QuadcopterPawn` OtherActor))
  (`KismetArrayLibrary.Array_Add` (`self.CapturedCopters`) _asquadcopter_pawn))

(event `self.BoostArea.OnComponentEndOverlap`
  (params (OverlappedComponent :type "PrimitiveComponent Object Reference") (OtherActor :type "Actor Object Reference") (OtherComp :type "PrimitiveComponent Object Reference") (OtherBodyIndex :type Integer))
  ;[1 1 1] Capturing Pawns Code
  (bind _asquadcopter_pawn (cast `/Game/Blueprints/Quadcopter/QuadcopterPawn` OtherActor))
  (`KismetArrayLibrary.Array_RemoveItem` (`self.CapturedCopters`) _asquadcopter_pawn))

(fn `CalculateBoostAmount`
  (params (Copter :type "/Game/Blueprints/Quadcopter/QuadcopterPawn Object Reference"))
  (returns (BoostAmount :type "Float (double-precision)"))
  (bind _boostarea (`self.BoostArea`))
  (return (* (/ (`KismetMathLibrary.VSize` (`KismetMathLibrary.ProjectVectorOnToVector` (- (+ (`SceneComponent.K2_GetComponentLocation` _boostarea) (* (`SceneComponent.GetUpVector` _boostarea) (`.OutHalfHeight` (`CapsuleComponent.GetScaledCapsuleSize` _boostarea)))) (`self.K2_GetActorLocation` Copter)) (`SceneComponent.GetUpVector` (`self.BoostArea`)))) (* 2.0 (`.OutHalfHeight` (`CapsuleComponent.GetScaledCapsuleSize` (`self.BoostArea`))))) (`self.MaxBoostFactor`))))

(fn `UserConstructionScript`)