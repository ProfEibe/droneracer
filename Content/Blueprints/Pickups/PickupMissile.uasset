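; Homing missile pickup for the drone racer that locks onto the player ahead of its owner, as reported by the game mode.
; Each tick it steers toward that drone with distance-scaled acceleration, integrates capped velocity with a swept move, and spins along its flight direction.
; Hitting a drone explodes, kills it and applies radial force within the blast radius; other hits release the target's lock and just explode.
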(event `self.ReceiveBeginPlay`
  ;[1 1 1] Initialization code
  (bind _asquadcopter_pawn (cast `/Game/Blueprints/Quadcopter/QuadcopterPawn` (`self.GetOwner`)))
  (bind _ascopter_controller (cast `/Game/Blueprints/Quadcopter/CopterController` (`Pawn.GetController` _asquadcopter_pawn)))
  (bind _asbp_drone_racer_gm (cast `/Game/GameMode/BP_DroneRacerGM` (`GameplayStatics.GetGameMode`)))
  (bind _playerinfront (`/Game/GameMode/BP_DroneRacerGM.GetPlayerInFront` _asbp_drone_racer_gm (`/Game/Blueprints/Quadcopter/CopterController.PlayerID` _ascopter_controller)))
  (bind _asquadcopter_pawn_2 (cast `/Game/Blueprints/Quadcopter/QuadcopterPawn` (`GameplayStatics.GetPlayerPawn` _playerinfront)))
  (bind _output_get (set `self.FollowedDrone` _asquadcopter_pawn_2))
  (`KismetArrayLibrary.Array_Add` (`/Game/Blueprints/Quadcopter/QuadcopterPawn.LockedOnMissiles` _output_get) self)
  (set `self.LinearVelocity` (* (`self.GetActorForwardVector`) (* (`self.MaxSpeed`) 0.3))))

(event `self.ReceiveTick`
  (params (DeltaSeconds :type "Float (single-precision)"))
  ;[1 1 1] Movement behaviour
  (`self.AdjustAcceleration`)
  (bind _vectortoplayer (`self.GetDirectionToPlayer`))
  (`self.Integrate` DeltaSeconds (* _vectortoplayer (`self.Acceleration`)))
  (`self.K2_SetActorRotation` (`KismetMathLibrary.MakeRotFromZ` (`self.LinearVelocity`)))
  (`self.AnimateSpin`))

(event `self.ReceiveHit`
  (params (MyComp :type "PrimitiveComponent Object Reference") (Other :type "Actor Object Reference") (OtherComp :type "PrimitiveComponent Object Reference") (bSelfMoved :type Boolean) (HitLocation :type "Vector Structure") (HitNormal :type "Vector Structure") (NormalImpulse :type "Vector Structure") (Hit :type "HitResult Structure (by ref)"))
  (bind _returnvalue (`self.K2_GetActorLocation`))
  ;[1 1 1] Missile hit behaviour
  (bind _asquadcopter_pawn (cast `/Game/Blueprints/Quadcopter/QuadcopterPawn` Other)
    (:`then`
      (`GameplayStatics.SpawnEmitterAtLocation` "/Game/ParticleEffects/ParticleTrail/ExplosionEffect.ExplosionEffect" (`self.K2_GetActorLocation`))
      (`/Game/Blueprints/Quadcopter/QuadcopterPawn.KillDrone` _asquadcopter_pawn self)
      (bind _allcoptersingame (`self.GetAllCopters`))
      (for _array_element _allcoptersingame
        (bind _returnvalue_2 (`KismetMathLibrary.VSize` (- (`self.K2_GetActorLocation` _array_element) _returnvalue)))
        (if (< _returnvalue_2 (`self.ExplosionRadius`))
          (`KismetSystemLibrary.PrintString` (`KismetStringLibrary.Conv_DoubleToString` _returnvalue_2) true false (struct :`R` 0.979645 :`G` 1.0 :`B` 0.878076 :`A` 1.0) 10.0)
          (`PrimitiveComponent.AddRadialForce` (`/Game/Blueprints/Quadcopter/QuadcopterPawn.CollisionBox` _array_element) _returnvalue (`self.ExplosionRadius`) (`self.ExplostionStrength`) "RIF_Constant" true)
          (`self.K2_DestroyActor`))))
    (:`CastFailed`
      (`KismetArrayLibrary.Array_RemoveItem` (`/Game/Blueprints/Quadcopter/QuadcopterPawn.LockedOnMissiles` (`self.FollowedDrone`)) self)
      (`self.KillMissile`))))

(fn `AdjustAcceleration`
  (bind _returnvalue (`KismetMathLibrary.Square` 100.0))
  (bind _returnvalue_2 (- (`KismetMathLibrary.Square` 1000.0) _returnvalue))
  (bind _returnvalue_3 (/ (- _returnvalue_2 (- (`KismetMathLibrary.VSizeSquared` (- (`self.K2_GetActorLocation` (`self.FollowedDrone`)) (`self.K2_GetActorLocation`))) _returnvalue)) _returnvalue_2))
  (if (< _returnvalue_3 0.0)
    (set `self.Acceleration` (`self.MinAcceleration`))
    (elif (> _returnvalue_3 1.0)
      (set `self.Acceleration` (`self.MaxSpeed`))
      (else
        (set `self.Acceleration` (* (`self.MaxAcceleration`) _returnvalue_3)) ; Set appropriate acceleration
      ))))

(fn `AnimateSpin`
  (bind _spinrotationangle (`self.SpinRotationAngle`))
  (`self.K2_AddActorLocalRotation` (`KismetMathLibrary.MakeRotator` 0.0 0.0 _spinrotationangle))
  (set `self.SpinRotationAngle` (+ _spinrotationangle (`self.SpinRotationSpeed`))))

(fn `GetAllCopters`
  (returns (AllCoptersInGame :type "Array of /Game/Blueprints/Quadcopter/QuadcopterPawn Object Reference"))
  (locals (AllCopters :type "Array of /Game/Blueprints/Quadcopter/QuadcopterPawn Object Reference"))
  (bind _allcopters (`local.AllCopters`))
  (bind _asbp_drone_racer_gm (cast `/Game/GameMode/BP_DroneRacerGM` (`GameplayStatics.GetGameMode`))
    (:`then`
      (bind _numberofplayers (`/Game/GameMode/BP_DroneRacerGM.GetNumberOfPlayers` _asbp_drone_racer_gm))
      (for _index (range _numberofplayers)
        (bind _asquadcopter_pawn (cast `/Game/Blueprints/Quadcopter/QuadcopterPawn` (`GameplayStatics.GetPlayerPawn` _index)))
        (`KismetArrayLibrary.Array_Add` _allcopters _asquadcopter_pawn)))
    (:`CastFailed`
      _))
  (return _allcopters))

(fn `GetDirectionToPlayer`
  (returns (VectorToPlayer :type "Vector Structure"))
  (return (`KismetMathLibrary.Normal` (- (`self.K2_GetActorLocation` (`self.FollowedDrone`)) (`self.K2_GetActorLocation`)))))

(fn `Integrate`
  (params (DeltaTime :type "Float (double-precision)") (LinearSteering :type "Vector Structure"))
  (bind _returnvalue (+ (`self.LinearVelocity`) (* LinearSteering DeltaTime)))
  (`self.K2_SetActorLocation` (+ (* (`self.LinearVelocity`) DeltaTime) (`self.K2_GetActorLocation`)) true)
  (if (> (`KismetMathLibrary.VSize` _returnvalue) (`self.MaxSpeed`))
    (set `self.LinearVelocity` (* (`KismetMathLibrary.Normal` _returnvalue) (`self.MaxSpeed`)))
    (else
      (set `self.LinearVelocity` _returnvalue))))

(fn `KillMissile`
  (`GameplayStatics.SpawnEmitterAtLocation` "/Game/ParticleEffects/ParticleTrail/ExplosionEffect.ExplosionEffect" (`self.K2_GetActorLocation`))
  (`self.K2_DestroyActor`))

(fn `UserConstructionScript`)