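; Magnet pickup effect that pulls its owning quadcopter to the next checkpoint, then along the level's track spline.
; Each tick, a seek-then-follow state machine moves the target slightly ahead on the spline, advancing by copter speed and wrapping at the end.
; A capped, distance-scaled pull is written to the copter's MovementAlteringDraw, and the target drives its magnet effect.
; The magnet is enabled on BeginPlay and disabled on EndPlay.
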(event `self.ReceiveBeginPlay`
  ;[1 1 1] Begin code
  (bind _asquadcopter_pawn (cast `/Game/Blueprints/Quadcopter/QuadcopterPawn` (`self.GetOwner`)))
  (bind _output_get (set `self.Copter` _asquadcopter_pawn))
  (bind _ascopter_controller (cast `/Game/Blueprints/Quadcopter/CopterController` (`Pawn.GetController` _output_get)))
  (set `self.CopterController` _ascopter_controller)
  (bind _outactors (`GameplayStatics.GetAllActorsOfClass` "/Game/Blueprints/Pickups/TrackSpline.TrackSpline_C"))
  (set `self.LevelSpline` (`/Game/Blueprints/Pickups/TrackSpline.Spline` (`KismetArrayLibrary.Array_Get` _outactors)))
  (bind _nextcheckpoint (`/Game/Blueprints/Quadcopter/CopterController.GetNextCheckpointActor` (`self.CopterController`)))
  (set `self.TargetLocation` (`self.K2_GetActorLocation` _nextcheckpoint))
  (`/Game/Blueprints/Quadcopter/QuadcopterPawn.EnableMagnet` (`self.Copter`)))

(event `self.ReceiveTick`
  (params (DeltaSeconds :type "Float (single-precision)"))
  (bind _levelspline (`self.LevelSpline`))
  (bind _returnvalue (- (`self.TargetLocation`) (`self.K2_GetActorLocation` (`self.Copter`))))
  (bind _returnvalue_2 (* _returnvalue 6.0))
  ;[1 1 1] Pull player along spline
  (switch `/Game/Blueprints/Pickups/MagnetSeekStage` (`self.SeekMode`)
    (:`NewEnumerator0`
      (bind _iscloseenough (`self.IsCloseToTarget` 300.0))
      (if _iscloseenough
        (set `self.CurrentSplineDistance` (`SplineComponent.GetDistanceAlongSplineAtSplinePoint` _levelspline (`KismetMathLibrary.FCeil` (`SplineComponent.FindInputKeyClosestToWorldLocation` _levelspline (`self.K2_GetActorLocation`)))))
        (set `self.SeekMode` "NewEnumerator1")))
    (:`NewEnumerator1`
      (set `self.CurrentSplineDistance` (`KismetMathLibrary.FMod` (+ (* (* (`KismetMathLibrary.VSize` (`/Game/Blueprints/Quadcopter/QuadcopterPawn.Velocity` (`self.Copter`))) 1.0) (* DeltaSeconds 1.0)) (`self.CurrentSplineDistance`)) (`SplineComponent.GetSplineLength` (`self.LevelSpline`))))
      (set `self.TargetLocation` (`SplineComponent.GetLocationAtDistanceAlongSpline` (`self.LevelSpline`) (+ (`self.CurrentSplineDistance`) 100.0) "World"))))
  (if (> (`KismetMathLibrary.VSizeSquared` _returnvalue_2) (`KismetMathLibrary.Square` 2500.0))
    (set `/Game/Blueprints/Quadcopter/QuadcopterPawn.MovementAlteringDraw` (* (`KismetMathLibrary.Normal` _returnvalue) 2000.0) (`self.Copter`))
    (else
      (set `/Game/Blueprints/Quadcopter/QuadcopterPawn.MovementAlteringDraw` _returnvalue_2 (`self.Copter`))))
  (`/Game/Blueprints/Quadcopter/QuadcopterPawn.UpdateMagnetTarget` (`self.Copter`) (`self.TargetLocation`)))

(event `self.ReceiveEndPlay`
  (params (EndPlayReason :type "EEndPlayReason Enum" :default "Destroyed"))
  ;[1 1 1] End code
  (`/Game/Blueprints/Quadcopter/QuadcopterPawn.DisableMagnet` (`self.Copter`)))

(fn `Integrate`
  (params (DeltaTime :type "Float (double-precision)") (LinearSteering :type "Vector Structure"))
  (bind _returnvalue (+ (`self.LinearVelocity`) (* LinearSteering DeltaTime)))
  (`self.K2_SetActorLocation` (`self.Copter`) (+ (* (`self.TargetLocation`) DeltaTime) (`self.K2_GetActorLocation`)) true false)
  (if (> (`KismetMathLibrary.VSize` _returnvalue) (`self.MaxSpeed`))
    (set `self.LinearVelocity` (* (`KismetMathLibrary.Normal` _returnvalue) (`self.MaxSpeed`)))
    (else
      (set `self.LinearVelocity` _returnvalue))))

(fn `IsCloseToTarget`
  (params (WhatIsClose :type "Float (double-precision)"))
  (returns (IsCloseEnough :type Boolean))
  (return (< (`KismetMathLibrary.VSize` (- (`self.TargetLocation`) (`self.K2_GetActorLocation` (`self.Copter`)))) WhatIsClose)))

(fn `SeekTarget`
  (params (DeltaTime :type "Float (double-precision)"))
  (`self.Integrate` DeltaTime (* (`KismetMathLibrary.Normal` (- (`self.TargetLocation`) (`self.K2_GetActorLocation`))) (`self.Acceleration`)))
  (return))

(fn `UserConstructionScript`)