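; Drone racer pickup placeholder that gives an overlapping quadcopter without a pickup either a preset item or a randomly chosen one.
; The random choice is weighted by race position and player count, using Missle, Net and Glass splines as per-pickup probability curves.
; A spawned PickupAnimator receives the chosen class and target copter.
; The placeholder then hides, disables collision and ticks down its respawn time before reappearing.
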(event `self.ReceiveBeginPlay`
  (bind _pickupsplines (`self.PickupSplines`))
  ;[1 1 1] Add Splines to Array at BeginPlay
  (`KismetArrayLibrary.Array_Add` _pickupsplines (`self.Missle`))
  (`KismetArrayLibrary.Array_Add` _pickupsplines (`self.Net`))
  (`KismetArrayLibrary.Array_Add` _pickupsplines (`self.Glass`)))

(event `self.ReceiveActorBeginOverlap`
  (params (OtherActor :type "Actor Object Reference"))
  ;[1 1 1] Pickup decision process
  (bind _asquadcopter_pawn (cast `/Game/Blueprints/Quadcopter/QuadcopterPawn` OtherActor))
  (if (== (`/Game/Blueprints/Quadcopter/QuadcopterPawn.HasPickup` _asquadcopter_pawn) false)
    (if (== (`self.PickupToGet`) -1)
      (bind _pickupindex (`self.DecidePickup` _asquadcopter_pawn))
      (`self.SetPickupToPlayer` _pickupindex _asquadcopter_pawn)
      (else
        (`self.SetPickupToPlayer` (`self.PickupToGet`) _asquadcopter_pawn)))
    (`self.SetPickupPlaceholderStatus` false)))

(event `self.ReceiveTick`
  (params (DeltaSeconds :type "Float (single-precision)"))
  ;[1 1 1] Cooldown if pawn collected pickup
  (bind _output_get (set `self.RespawnTimeLeft` (- (`self.RespawnTimeLeft`) DeltaSeconds)))
  (if (<= _output_get 0.0)
    (set `self.RespawnTimeLeft` (`self.RespawnTime`))
    (`self.SetPickupPlaceholderStatus` true)))

(fn `CreateAndEnableAnimator`
  (params (PickupClass :type "Actor Class Reference") (Quadcopter :type "/Game/Blueprints/Quadcopter/QuadcopterPawn Object Reference"))
  (bind _returnvalue (`|SpawnActorFromClass` "/Game/Blueprints/Pickups/PickupAnimator.PickupAnimator_C" (`self.GetTransform`) "Undefined" "OverrideRootScale" self))
  (set `/Game/Blueprints/Pickups/PickupAnimator.TargetCopter` Quadcopter _returnvalue)
  (set `/Game/Blueprints/Pickups/PickupAnimator.PickupClass` PickupClass _returnvalue)
  (cast `/Game/Blueprints/Quadcopter/CopterController` (`Pawn.GetController` Quadcopter))
  (`self.SetActorTickEnabled` _returnvalue true))

(fn `DecidePickup`
  (params (Pawn :type "/Game/Blueprints/Quadcopter/QuadcopterPawn Object Reference"))
  (returns (PickupIndex :type Integer))
  (locals (ChosenPickup :type Integer) (`p's` :type "Array of Float (double-precision)") (Sum :type "Float (double-precision)") (Random :type "Float (double-precision)"))
  ;[1 1 1] Get Number of Players and current Position
  (bind _ascopter_controller (cast `/Game/Blueprints/Quadcopter/CopterController` (`Pawn.GetController` Pawn))
    (:`then`
      (bind _asbp_drone_racer_gm (cast `/Game/GameMode/BP_DroneRacerGM` (`GameplayStatics.GetGameMode`))
        (:`then`
          (bind _position (`/Game/GameMode/BP_DroneRacerGM.GetPlayerPosition` _asbp_drone_racer_gm (`/Game/Blueprints/Quadcopter/CopterController.PlayerID` _ascopter_controller)))
          (bind _count (`/Game/GameMode/BP_DroneRacerGM.PlayerCountOnCircuit` _asbp_drone_racer_gm))
          (if (> _count 1)
            ;[1 1 1] Get p for each pickup
            (for _array_element (`self.PickupSplines`)
              (bind (_returnvalue_x _returnvalue_y _returnvalue_z) (`KismetMathLibrary.BreakVector` (`SplineComponent.GetLocationAtDistanceAlongSpline` _array_element (* (* (- _position 1) (/ 1.0 (`KismetMathLibrary.Conv_IntToDouble` (- _count 1)))) (`SplineComponent.GetSplineLength` _array_element)) "Local")))
              (`KismetArrayLibrary.Array_Add` (`local.p's`) _returnvalue_z))
            ;[1 1 1] Get Random Value
            (for _array_element_2 (`local.p's`)
              (bind _output_get (set `local.Sum` (+ (`local.Sum`) _array_element_2))))
            (set `local.Random` (`KismetMathLibrary.RandomFloatInRange` 0.0 _output_get))
            ;[1 1 1] Find final pickup
            (for (_array_element_3 _array_index) (`local.p's`)
              (bind _output_get_2 (set `local.Random` (- (`local.Random`) _array_element_3)))
              (if (< _output_get_2 0.0)
                (return _array_index) ; Just to get it working
              ))
            (return _array_index) ; Just to get it working
            (else
              (return 1) ; Case only 1 Player is left in Race
            )))
        (:`CastFailed`
          _)))
    (:`CastFailed`
      _))
  (`KismetSystemLibrary.PrintString` "CastFailed" false)
  (return 0))

(fn `SetPickupPlaceholderStatus`
  (params (IsActive :type Boolean))
  (`self.SetActorHiddenInGame` (not IsActive))
  (`self.SetActorEnableCollision` IsActive)
  (`self.SetActorTickEnabled` (not IsActive)))

(fn `SetPickupToPlayer`
  (params (Index :type Integer) (Pawn :type "/Game/Blueprints/Quadcopter/QuadcopterPawn Object Reference"))
  (set `/Game/Blueprints/Quadcopter/QuadcopterPawn.HasPickup` true Pawn)
  (`self.CreateAndEnableAnimator` (`KismetArrayLibrary.Array_Get` (`self.PossiblePickups`) Index) Pawn))

(fn `UserConstructionScript`)