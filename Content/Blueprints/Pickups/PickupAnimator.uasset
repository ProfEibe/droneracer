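; Short-lived actor that plays a roulette-style pickup animation on the HUD before granting a pickup to the target copter.
; BeginPlay copies the possible pickups from its PickupPlaceholder owner.
; Tick counts down two timers, cycling the displayed pickup at intervals and destroying the actor when the animation ends.
; Destroyed assigns the preset PickupClass to the copter, shows it on the HUD and flags the copter as holding a pickup.
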(event `self.ReceiveBeginPlay`
  (bind _aspickup_placeholder (cast `/Game/Blueprints/Pickups/PickupPlaceholder` (`self.GetOwner`)))
  (set `self.PossiblePickups` (`/Game/Blueprints/Pickups/PickupPlaceholder.PossiblePickups` _aspickup_placeholder)))

(event `self.ReceiveTick`
  (params (DeltaSeconds :type "Float (single-precision)"))
  (bind _output_get (set `self.AnimationTimeLeft` (- (`self.AnimationTimeLeft`) DeltaSeconds)))
  (if (> _output_get 0.0)
    (`self.LoopPickupAnimation` DeltaSeconds)
    (else
      (`self.K2_DestroyActor`))))

(event `self.ReceiveDestroyed`
  (bind _targetcopter (`self.TargetCopter`))
  (bind _output_get (set `/Game/Blueprints/Quadcopter/QuadcopterPawn.PickupClass` (`self.PickupClass`) _targetcopter))
  (`/Game/HUD/Player/PlayerHUD.DisplayPickup` (`self.TargetHUDWidget`) _output_get)
  (set `/Game/Blueprints/Quadcopter/QuadcopterPawn.HasPickup` true _targetcopter))

(fn `LoopPickupAnimation`
  (params (DeltaTime :type "Float (double-precision)"))
  (bind _output_get (set `self.TimeToNextDisplayLeft` (- (`self.TimeToNextDisplayLeft`) DeltaTime)))
  (if (<= _output_get 0.0)
    (set `self.TimeToNextDisplayLeft` (`self.TimeToNextDisplay`))
    (bind _result (`/Engine/EditorBlueprintResources/StandardMacros.IncrementInt` (`self.CurrentlyDisplayedPickupIndex`))
      (:`  `
        (bind _output_get_2 (set `self.CurrentlyDisplayedPickupIndex` (mod _result (`KismetArrayLibrary.Array_Length` (`self.PossiblePickups`)))))
        (`/Game/HUD/Player/PlayerHUD.DisplayPickup` (`self.TargetHUDWidget`) (`KismetArrayLibrary.Array_Get` (`self.PossiblePickups`) _output_get_2))))))

(fn `UserConstructionScript`)