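; Wall actor from the pickup set that plays a launch sound on spawn and breaks when a PickupMissile hits it.
; On such a hit it applies heavy damage and impulse to WallMesh, likely a destructible, and hides its particle system.
; Helpers for a timed lifetime and scale-up animation exist, but their calling graph never runs, so the wall neither grows nor expires by itself.
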(event `self.ReceiveBeginPlay`
  (`AkGameplayStatics.PostEventAtLocation` "/Game/Sounds/drone/drone_launch_wall.drone_launch_wall" (`self.K2_GetActorLocation`)))

(event `self.ReceiveHit`
  (params (MyComp :type "PrimitiveComponent Object Reference") (Other :type "Actor Object Reference") (OtherComp :type "PrimitiveComponent Object Reference") (bSelfMoved :type Boolean) (HitLocation :type "Vector Structure") (HitNormal :type "Vector Structure") (NormalImpulse :type "Vector Structure") (Hit :type "HitResult Structure (by ref)"))
  (cast `/Game/Blueprints/Pickups/PickupMissile` Other)
  (`DestructibleComponent.ApplyDamage` (`self.WallMesh`) 1000.0 HitLocation HitNormal 10000.0)
  (`SceneComponent.SetVisibility` (`self.ParticleSystem1`) false true))

(fn `DoAnimationCalculations`
  (params (DeltaTime :type "Float (double-precision)"))
  (returns (ScaleFactor :type "Float (double-precision)"))
  (bind _output_get (set `self.AnimationTime` (+ DeltaTime (`self.AnimationTime`))))
  (bind _returnvalue (/ _output_get (`self.AnimationDuration`)))
  (if (> _returnvalue 1.0)
    (return 1.0)
    (else
      (return _returnvalue))))

(fn `UserConstructionScript`)