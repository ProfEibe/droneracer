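; Glass pane pickup actor that plays a drone glass-launch sound on spawn and takes its owning quadcopter's player color when the player ID is nonzero.
; A hit from any quadcopter pawn applies heavy damage to the destructible pane, with impulse scaled by that pawn's speed.
; Fracturing plays a Wwise break sound and sets a lifespan so the shattered pane cleans itself up.
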(event `self.ReceiveBeginPlay`
  ;[1 1 1] Begin code
  (`AkGameplayStatics.PostEventAtLocation` "/Game/Sounds/drone/drone_launch_glass.drone_launch_glass" (`self.K2_GetActorLocation`))
  (bind _asquadcopter_pawn (cast `/Game/Blueprints/Quadcopter/QuadcopterPawn` (`self.GetOwner`)))
  (bind _playerid (`/Game/Blueprints/Quadcopter/QuadcopterPawn.PlayerId` _asquadcopter_pawn))
  (if (!= _playerid 0)
    (`PrimitiveComponent.SetMaterial` (`self.Plane`) 1 (`KismetArrayLibrary.Array_Get` (`self.GlassColors`) _playerid))))

(event `self.Plane.OnComponentFracture`
  (params (HitPoint :type "Vector Structure (by ref)") (HitDirection :type "Vector Structure (by ref)"))
  ;[1 1 1] OnFractureCode
  (`self.SetLifeSpan` (`self.TTL`))
  (`AkGameplayStatics.PostEventAtLocation` "/Game/Sounds/drone/glass_break.glass_break" (`self.K2_GetActorLocation`)))

(event `self.ReceiveHit`
  (params (MyComp :type "PrimitiveComponent Object Reference") (Other :type "Actor Object Reference") (OtherComp :type "PrimitiveComponent Object Reference") (bSelfMoved :type Boolean) (HitLocation :type "Vector Structure") (HitNormal :type "Vector Structure") (NormalImpulse :type "Vector Structure") (Hit :type "HitResult Structure (by ref)"))
  ;[1 1 1] OnHitCode
  (bind _asquadcopter_pawn (cast `/Game/Blueprints/Quadcopter/QuadcopterPawn` Other))
  (`DestructibleComponent.ApplyDamage` (`self.Plane`) 1000.0 HitLocation HitNormal (+ (* (`KismetMathLibrary.VSize` (`/Game/Blueprints/Quadcopter/QuadcopterPawn.Velocity` _asquadcopter_pawn)) 2.0) 1500.0)))

(fn `UserConstructionScript`)