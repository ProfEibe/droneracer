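; Breakable glass panel pickup actor that removes itself a set time after it fractures.
; On BeginPlay it shifts itself along its local X axis by a fixed offset.
; The Plane component's fracture event enables actor tick, which counts down TTL through DecrementTTL and destroys the actor once the value drops below zero.
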(event `self.ReceiveBeginPlay`
  (`self.K2_AddActorLocalOffset` (350.0 0.0 0.0)))

(event `self.Plane.OnComponentFracture`
  (params (HitPoint :type "Vector Structure (by ref)") (HitDirection :type "Vector Structure (by ref)"))
  (`self.SetActorTickEnabled` true))

(event `self.ReceiveTick`
  (params (DeltaSeconds :type "Float (single-precision)"))
  (bind _output_get (set `self.TTL` (- (`self.TTL`) DeltaSeconds)))
  (if (< _output_get 0.0)
    (`self.K2_DestroyActor`)))

(fn `UserConstructionScript`)