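; TrackSpline is a spline-driven track actor that builds a visible mesh along its Spline component.
; The construction script calls CreateMeshForSpline, which adds one spline mesh component per segment between consecutive points.
; Each piece attaches to Root with world transforms kept, takes world-space positions and tangents from its two points, and has a uniformly reduced cross-section.
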(fn `CreateMeshForSpline`
  (bind _spline (`self.Spline`))
  (for _index (range (+ (- (`SplineComponent.GetNumberOfSplinePoints` _spline) 2) 1))
    (bind _returnvalue (`AddComponent|NODE_AddSplineMeshComponent-0` :`bManualAttachment` true))
    (`SceneComponent.K2_AttachToComponent` _returnvalue (`self.Root`) "None" "KeepWorld" "KeepWorld" "KeepWorld" true)
    (bind (_location _tangent) (`SplineComponent.GetLocationAndTangentAtSplinePoint` _spline _index "World"))
    (bind (_location_2 _tangent_2) (`SplineComponent.GetLocationAndTangentAtSplinePoint` _spline (+ _index 1) "World"))
    (`SplineMeshComponent.SetStartAndEnd` _returnvalue _location _tangent _location_2 _tangent_2 true)
    (`SplineMeshComponent.SetStartScale` _returnvalue (0.3 0.3) true)
    (`SplineMeshComponent.SetEndScale` _returnvalue (0.3 0.3) true)))

(fn `UserConstructionScript`
  (`self.CreateMeshForSpline`))