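; PickupMissile is a homing missile that chases the first actor tagged "Target", cast to a Pawn.
; On BeginPlay it jumps forward from its spawn point and launches at max speed.
; Each tick it steers by manual velocity integration, accelerating harder as squared distance shrinks, though very close range uses MaxSpeed as acceleration.
; It aligns its Z axis to velocity with an added spin; overlap only prints a hit message.
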(event `self.ReceiveBeginPlay`
  (bind _returnvalue (`self.GetOwner`))
  (bind _rotation (.rotation (`self.GetTransform` _returnvalue)))
  ;[1 1 1] Get and save reference to specific player to follow
  (bind _outactors (`GameplayStatics.GetAllActorsWithTag` "Target"))
  (bind _aspawn (cast `Pawn` (`KismetArrayLibrary.Array_Get` _outactors)))
  (set `self.FollowedPlayer` _aspawn)
  (set `self.LinearVelocity` (* (`KismetMathLibrary.Normal` (`KismetMathLibrary.GetForwardVector` (`self.K2_GetActorRotation` _returnvalue))) (`self.MaxSpeed`)))
  (`self.K2_SetActorTransform` (`KismetMathLibrary.MakeTransform` (+ (* (`KismetMathLibrary.Normal` (`KismetMathLibrary.GetForwardVector` _rotation)) 500.0) (.location (`self.GetTransform` _returnvalue))) _rotation (.scale (`self.GetTransform` _returnvalue)))))

(event `self.ReceiveTick`
  (params (DeltaSeconds :type "Float (single-precision)"))
  ;[1 1 1] Movement behaviour
  (`self.AdjustAcceleration`)
  (bind _vectortoplayer (`self.GetDirectionToPlayer`))
  (`self.Integrate` DeltaSeconds (* _vectortoplayer (`self.Acceleration`)))
  (`self.K2_SetActorRotation` (`KismetMathLibrary.MakeRotFromZ` (`self.LinearVelocity`)))
  (`self.AnimateSpin`))

(event `self.ReceiveActorBeginOverlap`
  (params (OtherActor :type "Actor Object Reference"))
  (`KismetSystemLibrary.PrintString` "Rocket hit !!" true false (struct :`R` 1.0 :`B` 0.500452 :`A` 1.0) 20.0))

(fn `AdjustAcceleration`
  (bind _returnvalue (`KismetMathLibrary.Square` 100.0))
  (bind _returnvalue_2 (- (`KismetMathLibrary.Square` 1000.0) _returnvalue))
  (bind _returnvalue_3 (/ (- _returnvalue_2 (- (`KismetMathLibrary.VSizeSquared` (- (`self.K2_GetActorLocation` (`self.FollowedPlayer`)) (`self.K2_GetActorLocation`))) _returnvalue)) _returnvalue_2))
  (if (< _returnvalue_3 0.0)
    (set `self.Acceleration` (`self.MinAcceleration`))
    (elif (> _returnvalue_3 1.0)
      (set `self.Acceleration` (`self.MaxSpeed`))
      (else
        (set `self.Acceleration` (* (`self.MaxAcceleration`) _returnvalue_3)) ; Set appropriate acceleration
      ))))

(fn `AnimateSpin`
  (bind _spinrotationangle (`self.SpinRotationAngle`))
  (`self.K2_AddActorLocalRotation` (`KismetMathLibrary.MakeRotator` 0.0 0.0 _spinrotationangle))
  (set `self.SpinRotationAngle` (+ _spinrotationangle (`self.SpinRotationSpeed`))))

(fn `GetDirectionToPlayer`
  (returns (VectorToPlayer :type "Vector Structure"))
  (return (`KismetMathLibrary.Normal` (- (`self.K2_GetActorLocation` (`self.FollowedPlayer`)) (`self.K2_GetActorLocation`)))))

(fn `Integrate`
  (params (DeltaTime :type "Float (double-precision)") (LinearSteering :type "Vector Structure"))
  (bind _returnvalue (+ (`self.LinearVelocity`) (* LinearSteering DeltaTime)))
  (`self.K2_SetActorLocation` (+ (* (`self.LinearVelocity`) DeltaTime) (`self.K2_GetActorLocation`)))
  (if (> (`KismetMathLibrary.VSize` _returnvalue) (`self.MaxSpeed`))
    (set `self.LinearVelocity` (* (`KismetMathLibrary.Normal` _returnvalue) (`self.MaxSpeed`)))
    (else
      (set `self.LinearVelocity` _returnvalue))))

(fn `UserConstructionScript`)