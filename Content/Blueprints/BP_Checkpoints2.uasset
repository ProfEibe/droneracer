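; Lap-counting checkpoint Blueprint that relocates a single Trigger along three checkpoint components, CP0 to CP2.
; When an overlap with Trigger ends, it moves to the checkpoint indexed by CPCount and increments that count, with a DoOnce and short delay as debounce.
; At a count of three it instead waits, resets the count and increments Lap without moving Trigger.
; The MaxLaps check leads nowhere.
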(event `self.Trigger.OnComponentEndOverlap`
  (params (OverlappedComponent :type "PrimitiveComponent Object Reference") (OtherActor :type "Actor Object Reference") (OtherComp :type "PrimitiveComponent Object Reference") (OtherBodyIndex :type Integer))
  (bind _item (`KismetArrayLibrary.Array_Get` (`|MakeArray` (`self.CP_0`) (`self.CP_1`) (`self.CP_2`)) (`self.CP_Count`)))
  (if (== (`self.CP_Count`) 3)
    (`KismetSystemLibrary.Delay` 0.2)
    (set `self.CP_Count` 0)
    (set `self.Lap` (+ (`self.Lap`) 1))
    (if (<= (`self.Lap`) (`self.MaxLaps`))
      _)
    (else
      (`/Engine/EditorBlueprintResources/StandardMacros.DoOnce` false :!label _label
        (:`Completed`
          (`SceneComponent.K2_SetWorldLocationAndRotation` (`self.Trigger`) (`SceneComponent.K2_GetComponentLocation` _item) (`SceneComponent.K2_GetComponentRotation` _item) false false)
          (set `self.CP_Count` (+ (`self.CP_Count`) 1))
          (`KismetSystemLibrary.Delay` 0.2)
          (goto _label :!via `Reset`))))))

(fn `UserConstructionScript`)